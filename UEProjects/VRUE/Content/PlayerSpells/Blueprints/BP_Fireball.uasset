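; BP_Fireball is a VR player spell projectile that can be upgraded, intensified and launched at enemies.
; CastFireball spawns it at the camera, and IntensifyFireball grows its scale and light up to an intensity cap, setting boosted damage.
; LaunchFireball picks a slightly randomized direction from the right aim controller, and Tick moves it.
; Enemy overlap stops it and damages overlapping enemies, then Tick inflates it until a Niagara explosion and destruction.
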(event `Upgrade Fireball`
  (params (Value :type Integer))
  (set `self.Spell Default Damage` (* (/ (`KismetMathLibrary.Conv_IntToDouble` Value) 10.0) (`self.Spell Default Damage`)))
  (set `self.SpeedMultiplier` (* (`self.SpeedMultiplier`) Value)))

(event `Cast Fireball`
  (bind _returnvalue (`GameplayStatics.GetActorOfClass` "/Game/Player/VRPlayer.VRPlayer_C"))
  (`|SpawnActorFromClass` "BP_Fireball_C" (`KismetMathLibrary.MakeTransform` (`SceneComponent.K2_GetComponentLocation` (`/Game/Player/VRPlayer.Camera` _returnvalue))) "Undefined" "OverrideRootScale" null null))

(event `Intensify Fireball`
  (params (Intesifier :type Integer))
  (bind _spell_intensity (`self.Spell_Intensity`))
  (bind _pointlight (`self.PointLight`))
  (for _ (range (+ Intesifier 1))
    (if (< _spell_intensity (`self.Max_Spell_Intensity`))
      (set `self.Spell_Intensity` (+ _spell_intensity 100))
      (set `self.Spell_Damage` (* (`self.Spell Default Damage`) 1.1))
      (`self.SetActorScale3D` (+ (`self.GetActorScale3D`) (`self.Spell_Scale_Amount`)))
      (`PointLightComponent.SetSourceRadius` _pointlight (+ (`PointLightComponent.SourceRadius` _pointlight) 5.0))
      (`LocalLightComponent.SetAttenuationRadius` _pointlight (+ (`LocalLightComponent.AttenuationRadius` _pointlight) 5.0))
      (`LightComponent.SetIntensity` _pointlight (+ (`LightComponentBase.Intensity` _pointlight) 500.0))
      (`PointLightComponent.SetSourceLength` _pointlight (+ (`PointLightComponent.SourceLength` _pointlight) 20.0)))))

(event `Launch Fireball`
  (bind _returnvalue (`GameplayStatics.GetActorOfClass` "/Game/Player/VRPlayer.VRPlayer_C"))
  (set `self.Fireball_Destination` (`KismetMathLibrary.RandomUnitVectorInConeInDegrees` (`KismetMathLibrary.Conv_RotatorToVector` (`SceneComponent.K2_GetComponentRotation` (`/Game/Player/VRPlayer.MotionControllerRightAim` _returnvalue))) 1.0))
  (set `self.Fireball_Launched?` true)
  (`self.SetLifeSpan` 5.0))

(event `self.ReceiveTick`
  (params (DeltaSeconds :type "Float (single-precision)"))
  (bind (_returnvalue_x _returnvalue_y _returnvalue_z) (`KismetMathLibrary.BreakVector` (`self.GetActorScale3D`)))
  (bind _pointlight (`self.PointLight`))
  (if (`self.Fireball_Launched?`)
    (`self.K2_AddActorLocalOffset` (* (`self.Fireball_Destination`) (`self.SpeedMultiplier`)))
    (if (and (`self.Fireball_Exploding?`) (< _returnvalue_x 5.0))
      (`PointLightComponent.SetSourceRadius` _pointlight (+ (`PointLightComponent.SourceRadius` _pointlight) 20.0))
      (`LocalLightComponent.SetAttenuationRadius` _pointlight (+ (`LocalLightComponent.AttenuationRadius` _pointlight) 20.0))
      (`LightComponent.SetIntensity` _pointlight (+ (`LightComponentBase.Intensity` _pointlight) 0.0))
      (`PointLightComponent.SetSourceLength` _pointlight (+ (`PointLightComponent.SourceLength` _pointlight) 40.0))
      (`self.SetActorScale3D` (+ (`KismetMathLibrary.MakeVector` _returnvalue_x _returnvalue_y _returnvalue_z) (* (`self.Spell_Scale_Amount`) (2.0 2.0 2.0))))
      (elif (>= _returnvalue_x 5.0)
        (`/Engine/EditorBlueprintResources/StandardMacros.DoOnce` false
          (:`Completed`
            (`NiagaraFunctionLibrary.SpawnSystemAttached` "/Game/PlayerSpells/Effects/NS_FireBallExplosion.NS_FireBallExplosion" (`self.DefaultSceneRoot`) "None" (0.0 0.0 0.0) (struct) "KeepRelativeOffset")
            (`SceneComponent.SetVisibility` (`self.StaticMesh`) false false)
            (`SceneComponent.SetVisibility` (`self.PointLight`) false false)
            (`KismetSystemLibrary.Delay` 2.0)
            (`self.K2_DestroyActor`)))))))

(event `self.ReceiveBeginPlay`
  (bind _returnvalue (`GameplayStatics.GetActorOfClass` "/Game/Player/VRPlayer.VRPlayer_C"))
  (`PrimitiveComponent.IgnoreActorWhenMoving` (`self.SphereCollider`) _returnvalue false))

(event `self.SphereCollider.OnComponentBeginOverlap`
  (params (OverlappedComponent :type "PrimitiveComponent Object Reference") (OtherActor :type "Actor Object Reference") (OtherComp :type "PrimitiveComponent Object Reference") (OtherBodyIndex :type Integer) (bFromSweep :type Boolean) (SweepResult :type "HitResult Structure (by ref)"))
  (cast `/Game/Enemies/Blueprints/BP_EnemyClass` OtherActor)
  (set `self.Fireball_Exploding?` true)
  (set `self.SpeedMultiplier` (0.0 0.0 0.0))
  (`GameplayStatics.PlaySoundAtLocation` "/Game/Audio/Effects/SFX_Explosion01.SFX_Explosion01" (`SceneComponent.K2_GetComponentLocation` (`self.DefaultSceneRoot`)) (struct) 0.2 0.2 0.0 null null null null)
  (for _array_element (`PrimitiveComponent.GetOverlappingActors` (`self.SphereCollider`) "/Game/Enemies/Blueprints/BP_EnemyClass.BP_EnemyClass_C")
    (bind _asbp_enemy_class (cast `/Game/Enemies/Blueprints/BP_EnemyClass` _array_element))
    (`/Game/Enemies/Blueprints/BP_EnemyClass.Take damage` _asbp_enemy_class (`self.Spell_Damage`))))

(fn `UserConstructionScript`)