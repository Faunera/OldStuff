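; Player spell actor that gradually restores the VR player's health from a limited healing pool.
; CastHeal finds the player, fills the pool from HealAmount, and starts a Niagara effect and activation sound.
; Tick follows the player, moving a fixed, frame-rate-dependent amount from pool to health until empty or health reaches 100, then destroys the actor.
; UpgradeHeal scales HealAmount, while Intensify adds to the remaining pool.
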(event `Upgrade Heal`
  (params (Value :type Integer))
  (set `self.Heal Amount` (* (* (`KismetMathLibrary.Conv_IntToDouble` Value) 1.3) (`self.Heal Amount`))))

(event `Intensify`
  (params (Intensifier :type Integer))
  (for _ (range (+ Intensifier 1))
    (set `self.Healing Left` (+ (`self.Healing Left`) 10.0))))

(event `Cast Heal`
  (bind _returnvalue (`GameplayStatics.GetActorOfClass` "/Game/Player/VRPlayer.VRPlayer_C"))
  (set `self.Player Reference` _returnvalue)
  (set `self.Healing Left` (`self.Heal Amount`))
  (`AddComponent|NODE_AddNiagaraComponent-0`)
  (set `self.Healing?` true)
  (`GameplayStatics.PlaySound2D` "/Game/Audio/Effects/SFX_Heal_Activation.SFX_Heal_Activation" 1.0 1.0 0.0 null null))

(event `self.ReceiveTick`
  (params (DeltaSeconds :type "Float (single-precision)"))
  (bind _player_reference (`self.Player Reference`))
  (bind _playerhealth (`/Game/Player/VRPlayer.PlayerHealth` _player_reference))
  (`self.K2_SetActorLocation` (`self.K2_GetActorLocation` (`self.Player Reference`)))
  (if (and (`self.Healing?`) (< _playerhealth 100.0))
    (set `/Game/Player/VRPlayer.PlayerHealth` (+ _playerhealth (`self.HealPerTick`)) _player_reference)
    (set `self.Healing Left` (- (`self.Healing Left`) (`self.HealPerTick`)))
    (if (<= (`self.Healing Left`) 0.0)
      (set `self.Healing?` false :!label _label)
      (`self.K2_DestroyActor`))
    (elif (`self.Healing?`)
      (goto _label))))

(fn `UserConstructionScript`)