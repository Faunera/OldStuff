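; BP_Shield is a player spell shield actor that plays an activation sound and holds health until it breaks.
; It drains its own health every tick, unscaled by delta time, and destroys itself at zero.
; UpgradeShield sets a level-scaled lifespan and multiplies health, while Intensify adds health in repeated increments.
; On destruction it spawns BP_ShieldBreak at its transform.
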(event `self.ReceiveBeginPlay`
  (`GameplayStatics.PlaySoundAtLocation` "/Game/Audio/Effects/SFX_Shield_Activation.SFX_Shield_Activation" (`SceneComponent.K2_GetComponentLocation` (`self.DefaultSceneRoot`)) (struct) 1.0 1.0 0.0 null null null null))

(event `Upgrade Shield`
  (params (Value :type Integer))
  (`self.SetLifeSpan` (* (`KismetMathLibrary.Conv_IntToDouble` Value) 7.0))
  (set `self.Shield_Health` (* (`self.Shield_Health`) 1.3)))

(event `self.ReceiveTick`
  (params (DeltaSeconds :type "Float (single-precision)"))
  (`self.Damage shield` (`self.SelfDamageAmount`)))

(event `Damage shield`
  (params (`Damage Amount` :type "Float (double-precision)"))
  (bind _output_get (set `self.Shield_Health` (- (`self.Shield_Health`) `Damage Amount`)))
  (if (<= _output_get 0.0)
    (`self.K2_DestroyActor`)))

(event `self.ReceiveDestroyed`
  (`|SpawnActorFromClass` "/Game/Visual_Effects/Shield/BP_ShieldBreak.BP_ShieldBreak_C" (`SceneComponent.K2_GetComponentToWorld` (`self.DefaultSceneRoot`)) "Undefined" "OverrideRootScale" null null))

(event `Intensify`
  (params (Intensifier :type Integer))
  (for _ (range (+ Intensifier 1))
    (set `self.Shield_Health` (+ (`self.Shield_Health`) 20.0))))

(fn `UserConstructionScript`)