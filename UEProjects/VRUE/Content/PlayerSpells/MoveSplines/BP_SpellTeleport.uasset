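; BP_SpellTeleport is a player spell actor in the MoveSplines set, named for teleporting, though no teleport logic appears in its graph.
; Each Tick runs the parent logic, then sets CanActivateSpell once Points reaches zero or below.
; When that flag is set, ActivateSpell looks up the VRPlayer actor without using the result, then destroys the spell actor.
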(event `self.ReceiveTick`
  (params (DeltaSeconds :type "Float (single-precision)"))
  (`parent.ReceiveTick` DeltaSeconds)
  (if (<= (`self.Points`) 0)
    (set `self.Can Activate Spell` true)))

(event `self.Activate Spell`
  (if (`self.Can Activate Spell`)
    (`GameplayStatics.GetActorOfClass` "/Game/Player/VRPlayer.VRPlayer_C")
    (`self.K2_DestroyActor`)))

(fn `UserConstructionScript`
  (`parent.UserConstructionScript`))