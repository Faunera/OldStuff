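; BP_SpellFireBall is the fireball spell actor for the VR player, gated on completing goals from its parent class.
; When Points runs out, a resettable DoOnce in Tick unlocks activation and intensifying.
; Intensifying raises the level and creates new goals, blocking further intensifying until they are cleared.
; Activation spawns BP_Fireball at the VR camera, applies intensity, launches it, applies any stored upgrade, then destroys the spell actor.
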(event `self.ReceiveBeginPlay`
  (`parent.ReceiveBeginPlay`))

(event `self.ReceiveTick`
  (params (DeltaSeconds :type "Float (single-precision)"))
  (`parent.ReceiveTick` DeltaSeconds)
  (if (<= (`self.Points`) 0)
    (`/Engine/EditorBlueprintResources/StandardMacros.DoOnce` false :!label _label
      (:`Completed`
        (set `self.Can Activate Spell` true)
        (set `self.Can Intensify` true)))))

(event `self.Intensify Spell`
  (`GameplayStatics.PlaySound2D` "/Game/Audio/Effects/SFX_Intensify.SFX_Intensify" 1.0 1.0 0.0 null null)
  (if (and (`self.Can Activate Spell`) (`self.Can Intensify`))
    (set `self.Intesifier` (+ (`self.Intesifier`) 1))
    (`self.Create Goals`)
    (set `self.Can Intensify` false)
    (goto _label :!via `Reset`)
    (else
      (`KismetSystemLibrary.PrintString` "Failed Intesify"))))

(event `self.Activate Spell`
  (bind _intesifier (`self.Intesifier`))
  (if (`self.Can Activate Spell`)
    (bind _returnvalue (`GameplayStatics.GetActorOfClass` "/Game/Player/VRPlayer.VRPlayer_C"))
    (bind _returnvalue_2 (`|SpawnActorFromClass` "/Game/PlayerSpells/Blueprints/BP_Fireball.BP_Fireball_C" (`KismetMathLibrary.MakeTransform` (`SceneComponent.K2_GetComponentLocation` (`/Game/Player/VRPlayer.Camera` _returnvalue))) "Undefined" "OverrideRootScale" null null))
    (if (> _intesifier 0)
      (`/Game/PlayerSpells/Blueprints/BP_Fireball.Intensify Fireball` _returnvalue_2 _intesifier))
    (`/Game/PlayerSpells/Blueprints/BP_Fireball.Launch Fireball` _returnvalue_2)
    (if (`self.Upgraded`)
      (`/Game/PlayerSpells/Blueprints/BP_Fireball.Upgrade Fireball` _returnvalue_2 (`self.Up Value`)))
    (`self.K2_DestroyActor`)))

(event `self.Spell Upgrade`
  (params (Value :type Integer))
  (if (> Value 0)
    (set `self.Up Value` Value)
    (set `self.Upgraded` true)))

(fn `UserConstructionScript`
  (`parent.UserConstructionScript`))