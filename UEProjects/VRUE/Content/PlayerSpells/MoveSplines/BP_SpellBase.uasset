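; Base VR spell that lays out a spline path with goal actors, leaving activate, intensify and upgrade events empty.
; On BeginPlay it moves to the VRPlayer camera's position and yaw, nudges forward, then spawns a BP_SpellGoal at each spline point except the last.
; The construction script adds a thin, oriented spline mesh per segment; instanced-mesh placement is disconnected.
; Destroying the spell destroys its remaining goals.
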(event `self.ReceiveBeginPlay`
  (`self.SetActorScale3D` (1.0 1.0 1.0))
  ;[1 1 1] Get VRPlayer and set Splinespell rotation and location accordingly
  (bind _returnvalue (`GameplayStatics.GetActorOfClass` "/Game/Player/VRPlayer.VRPlayer_C"))
  (bind _camera (`/Game/Player/VRPlayer.Camera` _returnvalue))
  (bind (_returnvalue_roll _returnvalue_pitch _returnvalue_yaw) (`KismetMathLibrary.BreakRotator` (`SceneComponent.K2_GetComponentRotation` _camera)))
  (`SceneComponent.K2_SetWorldLocationAndRotation` (`self.DefaultSceneRoot`) (`SceneComponent.K2_GetComponentLocation` _camera) (`KismetMathLibrary.MakeRotator` 0.0 0.0 _returnvalue_yaw) false false)
  (`self.K2_AddActorLocalOffset` (25.0 0.0 0.0))
  ;[1 1 1] Add a SpellGoal to every spline point
  (`self.Create Goals`))

(event `self.ReceiveTick`
  (params (DeltaSeconds :type "Float (single-precision)")))

(event `Activate Spell`)

(event `Create Goals`
  (bind _spline (`self.Spline`))
  (for _index (range (+ (- (`SplineComponent.GetNumberOfSplinePoints` _spline) 2) 1))
    (bind _returnvalue (`|SpawnActorFromClass` "/Game/PlayerSpells/MoveSplines/BP_SpellGoal.BP_SpellGoal_C" (`KismetMathLibrary.MakeTransform` (`SplineComponent.GetLocationAtSplinePoint` _spline _index "World") (struct) (0.2 0.2 0.2)) "Undefined" "OverrideRootScale" null null))
    (`KismetArrayLibrary.Array_Add` (`self.Goals`) _returnvalue)
    (set `self.Points` (+ (`self.Points`) 1))))

(event `self.ReceiveDestroyed`
  (bind _goals (`self.Goals`))
  (if (`KismetArrayLibrary.Array_IsNotEmpty` _goals)
    (for _array_element _goals
      (if (`KismetSystemLibrary.IsValid` _array_element)
        (`self.K2_DestroyActor` _array_element)))))

(event `Intensify Spell`)

(event `Spell Upgrade`
  (params (Value :type Integer)))

(fn `UserConstructionScript`
  (for _index (range (+ (- (`SplineComponent.GetNumberOfSplinePoints` (`self.Spline`)) 2) 1))
    (bind _returnvalue (`SplineComponent.GetLocationAtSplinePoint` (`self.Spline`) _index "World"))
    (`AddComponent|NODE_AddSplineMeshComponent-0` :`RelativeTransform` (`KismetMathLibrary.MakeTransform` _returnvalue (`KismetMathLibrary.MakeRotFromY` (- (`SplineComponent.GetLocationAtSplinePoint` (`self.Spline`) (+ _index 1) "World") _returnvalue)) (0.01 0.22 0.01)))))