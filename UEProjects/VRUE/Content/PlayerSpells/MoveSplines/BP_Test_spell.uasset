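; BP_Test_spell is a test VR spell actor that, on BeginPlay, spawns a BP_SpellGoal 50 units below its Sphere.
; Grabbing it or overlapping the Sphere only prints debug text, and the construction script applies its Scale.
; Tick looks up the VRPlayer to cache camera pitch, but the camera-angle check and the player's Repeats increment are left disconnected.
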(event `self.ReceiveBeginPlay`
  (bind _output_get (set `self.GoalPosition` (- (`SceneComponent.K2_GetComponentLocation` (`self.Sphere`)) (0.0 0.0 50.0))))
  (`|SpawnActorFromClass` "/Game/PlayerSpells/MoveSplines/BP_SpellGoal.BP_SpellGoal_C" (`KismetMathLibrary.MakeTransform` _output_get (struct) (defaults `/Game/PlayerSpells/MoveSplines/BP_SpellGoal` "/Game/PlayerSpells/MoveSplines/BP_SpellGoal.BP_SpellGoal_C")) "Undefined" "OverrideRootScale" null null))

(event `self.GrabComponent.OnGrabbed`
  (`KismetSystemLibrary.PrintString` "Grabberu"))

(event `self.Sphere.OnComponentBeginOverlap`
  (params (OverlappedComponent :type "PrimitiveComponent Object Reference") (OtherActor :type "Actor Object Reference") (OtherComp :type "PrimitiveComponent Object Reference") (OtherBodyIndex :type Integer) (bFromSweep :type Boolean) (SweepResult :type "HitResult Structure (by ref)"))
  (bind _returnvalue (`GameplayStatics.GetActorOfClass` "/Game/Player/VRPlayer.VRPlayer_C"))
  (if true
    (`KismetSystemLibrary.PrintString` "Uwuuuuuu")
    (bind _returnvalue_2 (`GameplayStatics.GetActorOfClass` "/Game/Player/VRPlayer.VRPlayer_C"))))

(event `self.ReceiveTick`
  (params (DeltaSeconds :type "Float (single-precision)"))
  (bind _returnvalue (`GameplayStatics.GetActorOfClass` "/Game/Player/VRPlayer.VRPlayer_C"))
  (bind (_returnvalue_roll _returnvalue_pitch) (`KismetMathLibrary.BreakRotator` (`SceneComponent.K2_GetComponentRotation` (`/Game/Player/VRPlayer.Camera` _returnvalue))))
  (set `self.CameraRotation` _returnvalue_pitch))

(fn `UserConstructionScript`
  (`self.SetActorScale3D` (`self.Scale`)))