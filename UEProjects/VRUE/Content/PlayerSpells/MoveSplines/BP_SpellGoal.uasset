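; BP_SpellGoal is a touch target for spell casting that the VR player clears with either hand.
; When its Sphere begins an overlap, it checks whether the VRPlayer's LeftSphere or RightSphere overlaps it.
; On a hit, it finds a BP_SpellBase via GetActorOfClass, decrements that spell's Points and destroys itself if the spell is valid.
; The construction script sizes the actor from its Scale variable.
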(event `self.Sphere.OnComponentBeginOverlap`
  (params (OverlappedComponent :type "PrimitiveComponent Object Reference") (OtherActor :type "Actor Object Reference") (OtherComp :type "PrimitiveComponent Object Reference") (OtherBodyIndex :type Integer) (bFromSweep :type Boolean) (SweepResult :type "HitResult Structure (by ref)"))
  (bind _returnvalue (`GameplayStatics.GetActorOfClass` "/Game/Player/VRPlayer.VRPlayer_C"))
  (if (or (`PrimitiveComponent.IsOverlappingActor` (`/Game/Player/VRPlayer.LeftSphere` _returnvalue) self) (`PrimitiveComponent.IsOverlappingActor` (`/Game/Player/VRPlayer.RightSphere` _returnvalue) self))
    (bind _returnvalue_2 (`GameplayStatics.GetActorOfClass` "/Game/PlayerSpells/MoveSplines/BP_SpellBase.BP_SpellBase_C"))
    (`/Engine/EditorBlueprintResources/StandardMacros.IsValid` _returnvalue_2
      (:`Is Valid`
        (set `/Game/PlayerSpells/MoveSplines/BP_SpellBase.Points` (- (`/Game/PlayerSpells/MoveSplines/BP_SpellBase.Points` _returnvalue_2) 1) _returnvalue_2)
        (`self.K2_DestroyActor`)))))

(fn `UserConstructionScript`
  (`self.SetActorScale3D` (`self.Scale`)))