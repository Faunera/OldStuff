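; BP_BossTorch is the boss room intro trigger that lights torches in sequence, then spawns the boss.
; A player-tagged actor overlapping BoxCollider sets InBossRoom once.
; Tick then uses a short Delay to pace revealing BoxCollider's child components one by one by index.
; Once all are visible, it spawns a scaled-up BP_SmokeActor at the collider after a pause, followed shortly by an enlarged BP_Sloth.
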(event `self.ReceiveBeginPlay`)

(event `self.ReceiveTick`
  (params (DeltaSeconds :type "Float (single-precision)"))
  (bind _returnvalue (`SceneComponent.K2_GetComponentLocation` (`self.BoxCollider`)))
  (bind _returnvalue_2 (+ (`self.Index`) 1))
  (if (`self.InBossRoom?`)
    (`KismetSystemLibrary.Delay` 0.5)
    (if (not (`self.TorchesLit?`))
      (`SceneComponent.SetVisibility` (`SceneComponent.GetChildComponent` (`self.BoxCollider`) (`self.Index`)) true false)
      (set `self.Index` _returnvalue_2)
      (if (>= _returnvalue_2 9)
        (set `self.TorchesLit?` true)
        (`KismetSystemLibrary.Delay` 4.0)
        (`|SpawnActorFromClass` "/Game/Visual_Effects/Smoke/BP_SmokeActor.BP_SmokeActor_C" (`KismetMathLibrary.MakeTransform` _returnvalue (struct) (20.0 20.0 20.0)) "Undefined" "OverrideRootScale" null null)
        (`KismetSystemLibrary.Delay` 0.5)
        (`|SpawnActorFromClass` "/Game/Enemies/Blueprints/BP_Sloth.BP_Sloth_C" (`KismetMathLibrary.MakeTransform` _returnvalue (struct) (5.0 5.0 5.0)) "Undefined" "OverrideRootScale" null null)))))

(event `self.BoxCollider.OnComponentBeginOverlap`
  (params (OverlappedComponent :type "PrimitiveComponent Object Reference") (OtherActor :type "Actor Object Reference") (OtherComp :type "PrimitiveComponent Object Reference") (OtherBodyIndex :type Integer) (bFromSweep :type Boolean) (SweepResult :type "HitResult Structure (by ref)"))
  (if (`self.ActorHasTag` OtherActor "Player")
    (`/Engine/EditorBlueprintResources/StandardMacros.DoOnce` false
      (:`Completed`
        (set `self.InBossRoom?` true)))))

(fn `UserConstructionScript`)