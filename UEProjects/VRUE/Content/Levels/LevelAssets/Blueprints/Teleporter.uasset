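; Level teleporter actor that moves the VR player to a set location once it has been unlocked.
; CheckCount decrements OpenCount and, at zero or below, sets UnlockTP and adds a Niagara effect.
; Overlapping its box with an actor tagged Player while unlocked calls Teleport, which finds the VRPlayer by class and sets its location to TeleportLocation.
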(event `self.Box.OnComponentBeginOverlap`
  (params (OverlappedComponent :type "PrimitiveComponent Object Reference") (OtherActor :type "Actor Object Reference") (OtherComp :type "PrimitiveComponent Object Reference") (OtherBodyIndex :type Integer) (bFromSweep :type Boolean) (SweepResult :type "HitResult Structure (by ref)"))
  (if (and (`self.ActorHasTag` OtherActor "Player") (`self.UnlockTP`))
    (`self.Teleport`)))

(event `CheckCount`
  (bind _output_get (set `self.OpenCount` (- (`self.OpenCount`) 1)))
  (if (<= _output_get 0)
    (set `self.UnlockTP` true)
    (`AddComponent|NODE_AddNiagaraComponent-0`)))

(event `Teleport`
  (bind _returnvalue (`GameplayStatics.GetActorOfClass` "/Game/Player/VRPlayer.VRPlayer_C"))
  (`self.K2_SetActorLocationAndRotation` :`self` _returnvalue :`NewLocation` (`self.TeleportLocation`)))

(fn `UserConstructionScript`)