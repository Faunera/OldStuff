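; Tutorial prop that demonstrates a spell gesture with two hands looping through a downward motion.
; Each Tick lowers both hands by a fixed, frame-rate-dependent step, then snaps them back to raised start positions once the right hand reaches zero height.
; Hand collider overlaps hide the touched components, and each loop reset restores visibility to the root and all its children.
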(event `self.ReceiveBeginPlay`)

(event `self.ReceiveTick`
  (params (DeltaSeconds :type "Float (single-precision)"))
  (bind _righthand (`self.RightHand`))
  (bind (_relativelocation_x _relativelocation_y _relativelocation_z) (`KismetMathLibrary.BreakVector` (`SceneComponent.RelativeLocation` _righthand)))
  (`SceneComponent.K2_AddWorldOffset` (`self.LeftHand`) (0.0 0.0 -0.5) false false)
  (`SceneComponent.K2_AddWorldOffset` _righthand (0.0 0.0 -0.5) false false)
  (if (<= _relativelocation_z 0.0)
    (`SceneComponent.K2_SetRelativeLocation` (`self.LeftHand`) (60.0 -10.0 177.0) false false)
    (`SceneComponent.K2_SetRelativeLocation` (`self.RightHand`) (-60.0 10.0 170.0) false false)
    (`SceneComponent.SetVisibility` (`self.DefaultSceneRoot`) true true)))

(event `self.LeftHandCollider.OnComponentBeginOverlap`
  (params (OverlappedComponent :type "PrimitiveComponent Object Reference") (OtherActor :type "Actor Object Reference") (OtherComp :type "PrimitiveComponent Object Reference") (OtherBodyIndex :type Integer) (bFromSweep :type Boolean) (SweepResult :type "HitResult Structure (by ref)"))
  (`SceneComponent.SetVisibility` OtherComp false false))

(event `self.RightHandCollider.OnComponentBeginOverlap`
  (params (OverlappedComponent :type "PrimitiveComponent Object Reference") (OtherActor :type "Actor Object Reference") (OtherComp :type "PrimitiveComponent Object Reference") (OtherBodyIndex :type Integer) (bFromSweep :type Boolean) (SweepResult :type "HitResult Structure (by ref)"))
  (`SceneComponent.SetVisibility` OtherComp false false))

(fn `UserConstructionScript`)