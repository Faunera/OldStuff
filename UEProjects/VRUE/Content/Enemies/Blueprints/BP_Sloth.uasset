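; Sloth enemy character that wakes when AI perception senses the player, walks slowly and attacks with random montages.
; Perception writes line of sight and player to the Sloth_Controller blackboard; losing sight sets a zero-time timer intended to clear them.
; Head collider overlaps during attacks damage the VRPlayer, gated by a cooldown that nothing here decrements.
; Separate events trigger attacks and the looping sleep animation.
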(event `self.ReceiveBeginPlay`
  (bind _slothhealth (`self.SlothHealth`))
  (set `self.MaxHealth` _slothhealth)
  (set `self.Health` _slothhealth))

(event `self.AIPerception.OnTargetPerceptionUpdated`
  (params (Actor :type "Actor Object Reference") (Stimulus :type "AIStimulus Structure"))
  (if (and (`self.ActorHasTag` Actor "Player") (`.bSuccessfullySensed` (break `AIStimulus` Stimulus)))
    (`KismetSystemLibrary.K2_ClearAndInvalidateTimerHandle` (`self.EnemyTimer`))
    (bind _assloth_controller (cast `/Game/Enemies/Blueprints/Controllers/Sloth_Controller` (`self.GetController`)))
    (bind _blackboard (`AIController.Blackboard` _assloth_controller))
    (`BlackboardComponent.SetValueAsBool` _blackboard (`self.HasLineOfSight`) true)
    (`BlackboardComponent.SetValueAsObject` _blackboard (`self.PlayerObject`) Actor)
    (`self.Update Walk Speed` 0.0)
    (bind _returnvalue (`self.PlayAnimMontage` "/Game/Enemies/Meshes/Sloth/Sloth_Anim_Sloth_Skeleton_Sloth_WakeUp_Montage.Sloth_Anim_Sloth_Skeleton_Sloth_WakeUp_Montage"))
    (`KismetSystemLibrary.Delay` _returnvalue)
    (`self.Update Walk Speed` 50.0)
    (`SkeletalMeshComponent.PlayAnimation` (`self.Mesh`) "/Game/Enemies/Meshes/Sloth/Sloth_Anim_Sloth_Skeleton_Sloth_Walk_Montage.Sloth_Anim_Sloth_Skeleton_Sloth_Walk_Montage" true)
    (else
      (bind _returnvalue_2 (`KismetSystemLibrary.K2_SetTimerDelegate` (delegate `StartEnemyTimer`)))
      (set `self.EnemyTimer` _returnvalue_2))))

(event `StartEnemyTimer`
  (bind _assloth_controller (cast `/Game/Enemies/Blueprints/Controllers/Sloth_Controller` (`self.GetController`)))
  (bind _blackboard (`AIController.Blackboard` _assloth_controller))
  (`BlackboardComponent.SetValueAsBool` _blackboard (`self.HasLineOfSight`) false)
  (`BlackboardComponent.SetValueAsObject` _blackboard (`self.PlayerObject`) null))

(event `AttackPlayer`
  (bind _attackanims (`self.AttackAnims`))
  (set `self.IsAttacking` true)
  (bind _returnvalue (`self.PlayAnimMontage` (`|GetArrayItem` _attackanims (`KismetMathLibrary.RandomInteger` (`KismetArrayLibrary.Array_Length` _attackanims)))))
  (`KismetSystemLibrary.Delay` _returnvalue)
  (set `self.IsAttacking` false))

(event `self.HeadCollider.OnComponentBeginOverlap`
  (params (OverlappedComponent :type "PrimitiveComponent Object Reference") (OtherActor :type "Actor Object Reference") (OtherComp :type "PrimitiveComponent Object Reference") (OtherBodyIndex :type Integer) (bFromSweep :type Boolean) (SweepResult :type "HitResult Structure (by ref)"))
  (if (and (`self.IsAttacking`) (<= (`self.Attack Cooldown`) 0.0))
    (`KismetSystemLibrary.PrintString` "Sloth Hit Success")
    (bind _returnvalue (`GameplayStatics.GetActorOfClass` "/Game/Player/VRPlayer.VRPlayer_C"))
    (`/Game/Player/VRPlayer.Take Damage` _returnvalue (`self.Damage`) (0.0 0.0 0.0))
    (set `self.Attack Cooldown` 1.0)))

(event `Play sleep animation`
  (if (not (`self.Sleeping?`))
    (set `self.Sleeping?` true)
    (`SkeletalMeshComponent.PlayAnimation` (`self.Mesh`) "/Game/Enemies/Meshes/Sloth/Sloth_Anim_Sloth_Skeleton_Sloth_Sleep_Montage.Sloth_Anim_Sloth_Skeleton_Sloth_Sleep_Montage" true)))

(fn `Update Walk Speed`
  (params (NewWalkSpeed :type "Float (double-precision)"))
  (set `CharacterMovementComponent.MaxWalkSpeed` NewWalkSpeed (`self.CharacterMovement`))
  (`SkeletalMeshComponent.PlayAnimation` (`self.Mesh`) "/Game/Enemies/Meshes/Sloth/Sloth_Anim_Sloth_Skeleton_Sloth_Walk_Montage.Sloth_Anim_Sloth_Skeleton_Sloth_Walk_Montage" true))

(fn `UserConstructionScript`)