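; BP_EnemyClass is an enemy with health, a camera-facing health bar widget, an attack cooldown, and cast and random attack montages.
; Damage leads to Die, which plays a sound and notifies the Teleporter actors through CheckCount.
; Actor tags branch death: Boss also ends the level via BP_EndGate, while Respawn non-bosses refill health after a delay.
; Otherwise it drops an upgrade object and is destroyed, spawning smoke.
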(event `self.ReceiveBeginPlay`
  (set `self.Health` (`self.MaxHealth`))
  (bind _returnvalue (`|CreateWidget` "/Game/UI/Widgets/WBP_HealthBarWidget.WBP_HealthBarWidget_C"))
  (`WidgetComponent.SetWidget` (`self.Widget`) _returnvalue)
  (set `/Game/UI/Widgets/WBP_HealthBarWidget.Value` (`self.Health`) _returnvalue)
  (set `/Game/UI/Widgets/WBP_HealthBarWidget.MaxValue` (`self.MaxHealth`) _returnvalue)
  (set `self.HealthBar` _returnvalue))

(event `self.ReceiveTick`
  (params (DeltaSeconds :type "Float (single-precision)"))
  (bind _healthbar (`self.HealthBar`))
  (bind _widget (`self.Widget`))
  (set `self.Attack Cooldown` (- (`self.Attack Cooldown`) DeltaSeconds))
  (`SceneComponent.K2_SetWorldRotation` _widget (`KismetMathLibrary.FindLookAtRotation` (`SceneComponent.K2_GetComponentLocation` _widget) (`PlayerCameraManager.GetCameraLocation` (`GameplayStatics.GetPlayerCameraManager` 0))) false false)
  (if (`KismetSystemLibrary.IsValid` _healthbar)
    (set `/Game/UI/Widgets/WBP_HealthBarWidget.Value` (`self.Health`) _healthbar)))

(event `Take damage`
  (params (`Damage amount` :type "Float (double-precision)"))
  (bind _output_get (set `self.Health` (- (`self.Health`) `Damage amount`)))
  (if (<= _output_get 0.0)
    (`self.Die`)))

(event `Die`
  (bind _returnvalue (`GameplayStatics.GetActorOfClass` "/Game/Levels/LevelAssets/Blueprints/Teleporter.Teleporter_C"))
  (if (`KismetSystemLibrary.IsValid` _returnvalue)
    (`/Game/Levels/LevelAssets/Blueprints/Teleporter.CheckCount` _returnvalue)
    (bind _returnvalue_2 (`GameplayStatics.GetActorOfClass` "/Game/Levels/LevelAssets/Blueprints/Teleporter_2.Teleporter_2_C"))
    (`/Game/Levels/LevelAssets/Blueprints/Teleporter_2.CheckCount` _returnvalue_2))
  (`GameplayStatics.PlaySoundAtLocation` "/Game/Audio/Effects/SFX_Gobbo_Death.SFX_Gobbo_Death" (`self.K2_GetActorLocation`) (struct) 1.0 1.0 0.0 null null null null)
  (if (`self.ActorHasTag` "Boss")
    (bind _returnvalue_3 (`GameplayStatics.GetActorOfClass` "/Game/Levels/LevelAssets/Blueprints/BP_EndGate.BP_EndGate_C"))
    (`/Game/Levels/LevelAssets/Blueprints/BP_EndGate.End Level` _returnvalue_3)
    ;[1 1 1] Drop points for player
    (`|SpawnActorFromClass` "/Game/Player/BP_UpgradeObject.BP_UpgradeObject_C" (`KismetMathLibrary.MakeTransform` (`SceneComponent.K2_GetComponentLocation` (`self.CapsuleComponent`))) "Undefined" "OverrideRootScale" null null :!label _label)
    (`self.K2_DestroyActor`)
    (elif (`self.ActorHasTag` "Respawn")
      (`KismetSystemLibrary.Delay` 3.0)
      (set `self.Health` (`self.MaxHealth`))
      (else
        (goto _label)))))

(event `self.ReceiveDestroyed`
  (`|SpawnActorFromClass` "/Game/Visual_Effects/Smoke/BP_SmokeActor.BP_SmokeActor_C" (`KismetMathLibrary.MakeTransform` (`self.K2_GetActorLocation`)) "Undefined" "OverrideRootScale" null null))

(event `PlayCastAnimation`
  (bind _returnvalue (`self.PlayAnimMontage` "/Game/Models/RiggedGoblin/animations/NinjaLeftJab_Retargeted_Montage.NinjaLeftJab_Retargeted_Montage"))
  (`KismetSystemLibrary.Delay` _returnvalue))

(event `PlayAttackAnimation`
  (bind _attackanimations (`self.AttackAnimations`))
  (bind _returnvalue (`KismetMathLibrary.RandomInteger` (`KismetArrayLibrary.Array_Length` _attackanimations)))
  (set `self.IsAttacking` true)
  (if (`KismetArrayLibrary.Array_IsValidIndex` _attackanimations _returnvalue)
    (bind _returnvalue_2 (`self.PlayAnimMontage` (`|GetArrayItem` _attackanimations _returnvalue)))
    (`KismetSystemLibrary.Delay` _returnvalue_2)
    (set `self.IsAttacking` false)))

(fn `UserConstructionScript`)