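; BP_FireWizard is the Fire Wizard enemy character, which feeds AI perception results into its FireWizard_Controller's Blackboard.
; Sensing a Player-tagged actor cancels the lose-sight timer and sets HasLineOfSight and PlayerObject.
; Any other perception update starts a LineOfSightTimer countdown that clears both keys on expiry, delaying target loss.
; UpdateWalkSpeed exposes a setter for the movement component's max walk speed.
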(event `self.AIPerception.OnTargetPerceptionUpdated`
  (params (Actor :type "Actor Object Reference") (Stimulus :type "AIStimulus Structure"))
  (if (and (`self.ActorHasTag` Actor "Player") (`.bSuccessfullySensed` (break `AIStimulus` Stimulus)))
    (`KismetSystemLibrary.K2_ClearAndInvalidateTimerHandle` (`self.EnemyTimer`))
    (bind _asfire_wizard_controller (cast `/Game/Enemies/Blueprints/Controllers/FireWizard_Controller` (`self.GetController`)))
    (bind _blackboard (`AIController.Blackboard` _asfire_wizard_controller))
    (`BlackboardComponent.SetValueAsBool` _blackboard (`self.HasLineOfSight`) true)
    (`BlackboardComponent.SetValueAsObject` _blackboard (`self.PlayerObject`) Actor)
    (else
      (bind _returnvalue (`KismetSystemLibrary.K2_SetTimerDelegate` (delegate `StartEnemyTimer`) (`self.Line Of Sight Timer`)))
      (set `self.EnemyTimer` _returnvalue))))

(event `StartEnemyTimer`
  (bind _asfire_wizard_controller (cast `/Game/Enemies/Blueprints/Controllers/FireWizard_Controller` (`self.GetController`)))
  (bind _blackboard (`AIController.Blackboard` _asfire_wizard_controller))
  (`BlackboardComponent.SetValueAsBool` _blackboard (`self.HasLineOfSight`) false)
  (`BlackboardComponent.SetValueAsObject` _blackboard (`self.PlayerObject`) null))

(fn `Update Walk Speed`
  (params (NewWalkSpeed :type "Float (double-precision)"))
  (set `CharacterMovementComponent.MaxWalkSpeed` NewWalkSpeed (`self.CharacterMovement`)))

(fn `UserConstructionScript`)