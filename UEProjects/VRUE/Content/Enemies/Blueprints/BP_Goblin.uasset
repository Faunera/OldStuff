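; Goblin enemy character that spots the player through AI perception and deals melee damage to the VR player.
; Sighting plays an alert and writes the player to the GoblinController's blackboard; other perception updates start a timer that clears it.
; While attacking, hand and foot overlaps share one check against the player's capsule, applying damage, sound and a cooldown.
; A helper function sets walk speed.
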(event `self.AIPerception.OnTargetPerceptionUpdated`
  (params (Actor :type "Actor Object Reference") (Stimulus :type "AIStimulus Structure"))
  (if (and (`self.ActorHasTag` Actor "Player") (`.bSuccessfullySensed` (break `AIStimulus` Stimulus)))
    (`KismetSystemLibrary.K2_ClearAndInvalidateTimerHandle` (`self.EnemyTimer`))
    (bind _asgoblin_controller (cast `/Game/Enemies/Blueprints/Controllers/GoblinController` (`self.GetController`)))
    (bind _blackboard (`AIController.Blackboard` _asgoblin_controller))
    (`BlackboardComponent.SetValueAsBool` _blackboard (`self.HasLineOfSight`) true)
    (`BlackboardComponent.SetValueAsObject` _blackboard (`self.PlayerObject`) Actor)
    (`GameplayStatics.PlaySoundAtLocation` "/Game/Audio/Effects/SFX_Alert.SFX_Alert" (`self.K2_GetActorLocation`) (struct) 1.0 1.0 0.0 null null null null)
    (else
      (bind _returnvalue (`KismetSystemLibrary.K2_SetTimerDelegate` (delegate `StartEnemyTimer`) (`self.Line Of Sight Timer`)))
      (set `self.EnemyTimer` _returnvalue))))

(event `StartEnemyTimer`
  (bind _asgoblin_controller (cast `/Game/Enemies/Blueprints/Controllers/GoblinController` (`self.GetController`)))
  (bind _blackboard (`AIController.Blackboard` _asgoblin_controller))
  (`BlackboardComponent.SetValueAsBool` _blackboard (`self.HasLineOfSight`) false)
  (`BlackboardComponent.SetValueAsObject` _blackboard (`self.PlayerObject`) null))

(event `self.RightFoot.OnComponentBeginOverlap`
  (params (OverlappedComponent :type "PrimitiveComponent Object Reference") (OtherActor :type "Actor Object Reference") (OtherComp :type "PrimitiveComponent Object Reference") (OtherBodyIndex :type Integer) (bFromSweep :type Boolean) (SweepResult :type "HitResult Structure (by ref)"))
  (bind _returnvalue (`self.K2_GetActorLocation`))
  (if (`self.IsAttacking`) :!label _label
    (if (<= (`self.Attack Cooldown`) 0.0)
      (bind _returnvalue_2 (`GameplayStatics.GetActorOfClass` "/Game/Player/VRPlayer.VRPlayer_C"))
      (bind _capsule (`/Game/Player/VRPlayer.Capsule` _returnvalue_2))
      (if (or (`PrimitiveComponent.IsOverlappingComponent` _capsule (`self.LeftHand`)) (`PrimitiveComponent.IsOverlappingComponent` _capsule (`self.RightHand`)) (`PrimitiveComponent.IsOverlappingComponent` _capsule (`self.LeftFoot`)) (`PrimitiveComponent.IsOverlappingComponent` _capsule (`self.RightFoot`)))
        (`/Game/Player/VRPlayer.Take Damage` _returnvalue_2 (`self.Damage`) _returnvalue)
        (`GameplayStatics.PlaySoundAtLocation` "/Game/Audio/Effects/SFX_Gobbo_Hit.SFX_Gobbo_Hit" _returnvalue (struct) 1.0 1.0 0.0 null null null null)
        (set `self.Attack Cooldown` 1.0)))))

(event `self.LeftFoot.OnComponentBeginOverlap`
  (params (OverlappedComponent :type "PrimitiveComponent Object Reference") (OtherActor :type "Actor Object Reference") (OtherComp :type "PrimitiveComponent Object Reference") (OtherBodyIndex :type Integer) (bFromSweep :type Boolean) (SweepResult :type "HitResult Structure (by ref)"))
  (goto _label))

(event `self.RightHand.OnComponentBeginOverlap`
  (params (OverlappedComponent :type "PrimitiveComponent Object Reference") (OtherActor :type "Actor Object Reference") (OtherComp :type "PrimitiveComponent Object Reference") (OtherBodyIndex :type Integer) (bFromSweep :type Boolean) (SweepResult :type "HitResult Structure (by ref)"))
  (goto _label))

(event `self.LeftHand.OnComponentBeginOverlap`
  (params (OverlappedComponent :type "PrimitiveComponent Object Reference") (OtherActor :type "Actor Object Reference") (OtherComp :type "PrimitiveComponent Object Reference") (OtherBodyIndex :type Integer) (bFromSweep :type Boolean) (SweepResult :type "HitResult Structure (by ref)"))
  (goto _label))

(fn `Update Walk Speed`
  (params (NewWalkSpeed :type "Float (double-precision)"))
  (set `CharacterMovementComponent.MaxWalkSpeed` NewWalkSpeed (`self.CharacterMovement`)))

(fn `UserConstructionScript`)