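; Behavior tree task that makes the Frost Wizard cast a ring of icicle projectiles.
; After a brief delay, it spawns icicle actors at evenly stepped yaw angles on a radius around the wizard's SpellSpawn point.
; Each starts at zero scale, takes the spawn point's yaw and selects its own movement direction.
; The task finishes successfully once the loop completes, without waiting on the icicles.
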(event `self.ReceiveExecuteAI`
  (params (OwnerController :type "AIController Object Reference") (ControlledPawn :type "Pawn Object Reference"))
  (bind _spellamount (`self.SpellAmount`))
  (bind _asbp_frost_wizard (cast `/Game/Enemies/Blueprints/BP_FrostWizard` ControlledPawn))
  (`KismetSystemLibrary.Delay` 0.1)
  (for _index (range (+ _spellamount 1))
    (bind _spellspawn (`/Game/Enemies/Blueprints/BP_FrostWizard.SpellSpawn` _asbp_frost_wizard))
    (bind _returnvalue (`|SpawnActorFromClass` "/Game/Enemies/Projectiles/Blueprints/BP_Wizard_Icicle.BP_Wizard_Icicle_C" (`KismetMathLibrary.Conv_VectorToTransform` (+ (* (`KismetMathLibrary.GetForwardVector` (`KismetMathLibrary.MakeRotator` 0.0 0.0 (`KismetMathLibrary.Conv_IntToDouble` (* _index (/ 360 _spellamount))))) (`self.Radius`)) (`SceneComponent.K2_GetComponentLocation` _spellspawn))) "Undefined" "OverrideRootScale" null null))
    (`Actor.SetActorScale3D` _returnvalue (0.0 0.0 0.0))
    (bind (_returnvalue_roll _returnvalue_pitch _returnvalue_yaw) (`KismetMathLibrary.BreakRotator` (`SceneComponent.K2_GetComponentRotation` _spellspawn)))
    (`Actor.K2_SetActorRotation` _returnvalue (`KismetMathLibrary.MakeRotator` 0.0 0.0 _returnvalue_yaw) false)
    (`/Game/Enemies/Projectiles/Blueprints/BP_Wizard_Icicle.Select Movement Direction` _returnvalue))
  (`self.FinishExecute` true))