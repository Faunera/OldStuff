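; Behavior tree task that picks a ranged chase destination around the BP_FrostWizard actor for the controlled pawn.
; On execute, it queries a random reachable point within MovementRadius of the wizard and writes it to the RangedChaseLocation blackboard key.
; If no point is found, it writes the pawn's current location instead.
; It only sets the key and finishes successfully, without moving the pawn.
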(event `self.ReceiveExecuteAI`
  (params (OwnerController :type "AIController Object Reference") (ControlledPawn :type "Pawn Object Reference"))
  (bind _returnvalue (`GameplayStatics.GetActorOfClass` "/Game/Enemies/Blueprints/BP_FrostWizard.BP_FrostWizard_C"))
  (bind (_randomlocation _returnvalue_2) (`NavigationSystemV1.K2_GetRandomReachablePointInRadius` (`Actor.K2_GetActorLocation` _returnvalue) (`self.MovementRadius`) null null))
  (if _returnvalue_2
    (`BTFunctionLibrary.SetBlackboardValueAsVector` (`self.RangedChaseLocation`) _randomlocation)
    (else
      (`BTFunctionLibrary.SetBlackboardValueAsVector` (`self.RangedChaseLocation`) (`Actor.K2_GetActorLocation` ControlledPawn))))
  (`self.FinishExecute` true))