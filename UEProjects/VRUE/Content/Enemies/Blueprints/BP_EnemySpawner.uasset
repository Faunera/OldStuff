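; Trigger actor that spawns an AI enemy when an actor tagged Player overlaps it.
; The pawn gets a configurable class and behavior tree, faces the player camera, and receives an Enemy tag, secondary tag and configured scale.
; After spawning, the overlap event destroys every BP_EnemySpawner in the level, itself included.
; SpawnEnemyFunction repeats the spawn logic without that cleanup and is not called within this Blueprint.
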(event `self.ReceiveActorBeginOverlap`
  (params (OtherActor :type "Actor Object Reference"))
  (if (`self.ActorHasTag` OtherActor "Player")
    (bind _returnvalue (`AIBlueprintHelperLibrary.SpawnAIFromClass` (`self.Pawn Class`) (`self.Behavior Tree`) (`self.Spawn Transform Location`) (`KismetMathLibrary.FindLookAtRotation` (`self.Spawn Transform Location`) (`PlayerCameraManager.GetCameraLocation` (`GameplayStatics.GetPlayerCameraManager` 0))) false null))
    (set `Actor.Tags` (`|MakeArray` "Enemy" (`self.Secondary Tag`)) _returnvalue)
    (`self.SetActorScale3D` _returnvalue (`self.Spawn Transform Scale`))
    (bind _outactors (`GameplayStatics.GetAllActorsOfClass` "BP_EnemySpawner_C"))
    (for _array_element _outactors
      (`self.K2_DestroyActor` _array_element))))

(fn `Spawn Enemy Function`
  (bind _returnvalue (`AIBlueprintHelperLibrary.SpawnAIFromClass` (`self.Pawn Class`) (`self.Behavior Tree`) (`self.Spawn Transform Location`) (`KismetMathLibrary.FindLookAtRotation` (`self.Spawn Transform Location`) (`PlayerCameraManager.GetCameraLocation` (`GameplayStatics.GetPlayerCameraManager` 0))) false null))
  (set `Actor.Tags` (`|MakeArray` "Enemy" (`self.Secondary Tag`)) _returnvalue)
  (`self.SetActorScale3D` _returnvalue (`self.Spawn Transform Scale`)))

(fn `UserConstructionScript`)