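; Fireball projectile of the fire wizard that damages the VR player or their shield.
; SelectMovementDirection picks a random direction in a narrow cone around the wizard's forward, and Tick moves the actor along it.
; Overlapping player or shield stops it and applies damage, prioritising the player.
; Tick then grows mesh and light until final scale, when it spawns a Niagara explosion, hides and self-destroys after a delay.
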(event `Select Movement Direction`
  (bind _returnvalue (`GameplayStatics.GetActorOfClass` "/Game/Enemies/Blueprints/BP_FireWizard.BP_FireWizard_C"))
  (bind (_returnvalue_x _returnvalue_y) (`KismetMathLibrary.BreakVector` (`self.GetActorForwardVector` _returnvalue)))
  (set `self.Projectile goal` (`KismetMathLibrary.RandomUnitVectorInConeInDegrees` (`KismetMathLibrary.MakeVector` _returnvalue_x _returnvalue_y) 15.0)))

(event `self.ReceiveTick`
  (params (DeltaSeconds :type "Float (single-precision)"))
  (bind (_returnvalue_x _returnvalue_y _returnvalue_z) (`KismetMathLibrary.BreakVector` (`self.GetActorScale3D`)))
  (bind _pointlight (`self.PointLight`))
  (`self.K2_AddActorLocalOffset` (* (`self.Projectile goal`) (`self.Projectile speed`)))
  (if (and (`self.Fireball Exploding?`) (< _returnvalue_x (`self.Final Scale`)))
    (`PointLightComponent.SetSourceRadius` _pointlight (+ (`PointLightComponent.SourceRadius` _pointlight) 20.0))
    (`LocalLightComponent.SetAttenuationRadius` _pointlight (+ (`LocalLightComponent.AttenuationRadius` _pointlight) 20.0))
    (`LightComponent.SetIntensity` _pointlight (+ (`LightComponentBase.Intensity` _pointlight) 0.0))
    (`PointLightComponent.SetSourceLength` _pointlight (+ (`PointLightComponent.SourceLength` _pointlight) 40.0))
    (`self.SetActorScale3D` (+ (`KismetMathLibrary.MakeVector` _returnvalue_x _returnvalue_y _returnvalue_z) (* (`self.Spell Scale Amount`) (2.0 2.0 2.0))))
    (elif (>= _returnvalue_x (`self.Final Scale`))
      (`/Engine/EditorBlueprintResources/StandardMacros.DoOnce` false
        (:`Completed`
          (`NiagaraFunctionLibrary.SpawnSystemAttached` "/Game/Enemies/Projectiles/Visual_Effects/NS_WizardFireBallExplosion.NS_WizardFireBallExplosion" (`self.DefaultSceneRoot`) "None" (0.0 0.0 0.0) (struct) "KeepRelativeOffset")
          (`SceneComponent.SetVisibility` (`self.StaticMesh`) false false)
          (`SceneComponent.SetVisibility` (`self.PointLight`) false false)
          (`KismetSystemLibrary.Delay` 2.0)
          (`self.K2_DestroyActor`))))))

(event `self.SphereCollider.OnComponentBeginOverlap`
  (params (OverlappedComponent :type "PrimitiveComponent Object Reference") (OtherActor :type "Actor Object Reference") (OtherComp :type "PrimitiveComponent Object Reference") (OtherBodyIndex :type Integer) (bFromSweep :type Boolean) (SweepResult :type "HitResult Structure (by ref)"))
  (bind _returnvalue (`ActorComponent.GetOwner` (`self.SphereCollider`)))
  (cast `/Game/PlayerSpells/Blueprints/BP_Shield` OtherActor
    (:`then`
      _)
    (:`CastFailed`
      (cast `/Game/Player/VRPlayer` OtherActor)))
  (set `self.Fireball Exploding?` true)
  (set `self.Projectile speed` (0.0 0.0 0.0))
  (bind _returnvalue_2 (`GameplayStatics.GetActorOfClass` "/Game/Player/VRPlayer.VRPlayer_C"))
  (if (`PrimitiveComponent.IsOverlappingActor` (`/Game/Player/VRPlayer.Capsule` _returnvalue_2) _returnvalue)
    (`/Engine/EditorBlueprintResources/StandardMacros.DoOnce` false
      (:`Completed`
        (`/Game/Player/VRPlayer.Take Damage` _returnvalue_2 (`self.Spell Damage`) (`SceneComponent.K2_GetComponentLocation` (`self.DefaultSceneRoot`)))))
    (else
      (bind _returnvalue_3 (`GameplayStatics.GetActorOfClass` "/Game/PlayerSpells/Blueprints/BP_Shield.BP_Shield_C"))
      (`/Engine/EditorBlueprintResources/StandardMacros.IsValid` _returnvalue_3
        (:`Is Valid`
          (if (`self.IsOverlappingActor` _returnvalue_3 _returnvalue)
            (`/Game/PlayerSpells/Blueprints/BP_Shield.Damage shield` _returnvalue_3 (`self.Spell Damage`))))))))

(event `self.ReceiveBeginPlay`
  (bind _returnvalue (`GameplayStatics.GetActorOfClass` "BP_Wizard_Fireball_C"))
  (`PrimitiveComponent.IgnoreActorWhenMoving` (`self.SphereCollider`) _returnvalue true))

(fn `UserConstructionScript`)