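; Frost wizard icicle projectile that damages the VR player or their shield.
; Each Tick grows it until large enough, then triggers the wizard's cast animation and moves it by a frame-rate-dependent offset, spinning and shrinking.
; SelectMovementDirection aims it along the wizard's forward vector with minimal spread.
; Hitting player or shield, or shrinking away, hides and disarms it before delayed destruction and a counter-gated garbage collection.
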(event `Select Movement Direction`
  (bind _returnvalue (`GameplayStatics.GetActorOfClass` "/Game/Enemies/Blueprints/BP_FrostWizard.BP_FrostWizard_C"))
  (bind (_returnvalue_x _returnvalue_y) (`KismetMathLibrary.BreakVector` (`self.GetActorForwardVector` _returnvalue)))
  (set `self.Projectile goal` (`KismetMathLibrary.RandomUnitVectorInConeInDegrees` (`KismetMathLibrary.MakeVector` _returnvalue_x _returnvalue_y) 0.1)))

(event `self.ReceiveTick`
  (params (DeltaSeconds :type "Float (single-precision)"))
  (bind _defaultsceneroot (`self.DefaultSceneRoot`))
  (bind _garbage_collection (`self.Garbage collection`))
  (bind _defaultsceneroot_2 (`self.DefaultSceneRoot`))
  (bind _returnvalue_x (`KismetMathLibrary.BreakVector` (`SceneComponent.K2_GetComponentScale` _defaultsceneroot_2)))
  (bind (_returnvalue_x_2 _returnvalue_y _returnvalue_z) (`KismetMathLibrary.BreakVector` (+ (`SceneComponent.RelativeScale3D` _defaultsceneroot_2) (`self.Scale offset`))))
  (bind (_returnvalue_x_3 _returnvalue_y_2 _returnvalue_z_2) (`KismetMathLibrary.BreakVector` (- (`SceneComponent.K2_GetComponentScale` _defaultsceneroot) (`self.Scale offset`))))
  (if (`self.Launched?`)
    (`self.K2_AddActorWorldOffset` (* (`self.Projectile goal`) (`self.Spell speed`)) :!label _label)
    (`/Engine/EditorBlueprintResources/StandardMacros.IsValid` _defaultsceneroot
      (:`Is Valid`
        (`SceneComponent.K2_AddRelativeRotation` _defaultsceneroot (struct :`Roll` 20.0) false false)
        (`/Engine/EditorBlueprintResources/StandardMacros.IsValid` _defaultsceneroot
          (:`Is Valid`
            (`SceneComponent.SetRelativeScale3D` _defaultsceneroot (`KismetMathLibrary.MakeVector` _returnvalue_x_3 _returnvalue_y_2 _returnvalue_z_2))
            (if (<= _returnvalue_z_2 0.1)
              (`KismetSystemLibrary.Delay` 0.5)
              (`SceneComponent.SetVisibility` (`self.StaticMesh`) false false :!label _label_2)
              (set `self.Spell Damage` 0.0)
              (`KismetSystemLibrary.Delay` 1.5)
              (`self.K2_DestroyActor`)
              (if (>= _garbage_collection 5)
                (`KismetSystemLibrary.CollectGarbage`)
                (set `self.Garbage collection` 0)
                (else
                  (set `self.Garbage collection` (+ _garbage_collection 1)))))))))
    (else
      (`SceneComponent.SetRelativeScale3D` _defaultsceneroot_2 (`KismetMathLibrary.MakeVector` _returnvalue_x_2 _returnvalue_y _returnvalue_z))
      (if (>= _returnvalue_x 0.5)
        (bind _returnvalue (`GameplayStatics.GetActorOfClass` "/Game/Enemies/Blueprints/BP_FrostWizard.BP_FrostWizard_C"))
        (`/Game/Enemies/Blueprints/BP_EnemyClass.PlayCastAnimation` _returnvalue)
        (set `self.Launched?` true)
        (goto _label)))))

(event `self.CapsuleCollider.OnComponentBeginOverlap`
  (params (OverlappedComponent :type "PrimitiveComponent Object Reference") (OtherActor :type "Actor Object Reference") (OtherComp :type "PrimitiveComponent Object Reference") (OtherBodyIndex :type Integer) (bFromSweep :type Boolean) (SweepResult :type "HitResult Structure (by ref)"))
  (bind _returnvalue (`ActorComponent.GetOwner` (`self.CapsuleCollider`)))
  (bind _returnvalue_2 (`GameplayStatics.GetActorOfClass` "/Game/Player/VRPlayer.VRPlayer_C"))
  (if (`self.IsOverlappingActor` _returnvalue_2 _returnvalue)
    (`/Engine/EditorBlueprintResources/StandardMacros.DoOnce` false
      (:`Completed`
        (`/Game/Player/VRPlayer.Take Damage` _returnvalue_2 (`self.Spell Damage`) (`SceneComponent.K2_GetComponentLocation` (`self.DefaultSceneRoot`)))
        (goto _label_2)))
    (else
      (bind _returnvalue_3 (`GameplayStatics.GetActorOfClass` "/Game/PlayerSpells/Blueprints/BP_Shield.BP_Shield_C"))
      (`/Engine/EditorBlueprintResources/StandardMacros.IsValid` _returnvalue_3
        (:`Is Valid`
          (if (`self.IsOverlappingActor` _returnvalue_3 _returnvalue)
            (`/Game/PlayerSpells/Blueprints/BP_Shield.Damage shield` _returnvalue_3 (`self.Spell Damage`))
            (goto _label_2)))))))

(fn `UserConstructionScript`)