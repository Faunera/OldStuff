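; BP_Interactable is an interactable prop Blueprint that plays a sound when it is interacted with or picked up.
; The Interact and Pickup events each play the same Sound variable in 2D, with volume taken from the game instance's AudioVolume scaled from a percentage.
; Neither event has other logic, the player reference passed to Pickup is unused, and the construction script is empty.
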(event `Interact`
  (bind _asbp_game_instance (cast `/Game/Data/BP_GameInstance` (`GameplayStatics.GetGameInstance`)))
  (`GameplayStatics.PlaySound2D` (`self.Sound`) (* (`/Game/Data/BP_GameInstance.AudioVolume` _asbp_game_instance) 0.01) 1.0 0.0 null null))

(event `Pickup`
  (params (`Player Reference` :type "/Game/Player/Blueprints/BP_Player Object Reference"))
  (bind _asbp_game_instance (cast `/Game/Data/BP_GameInstance` (`GameplayStatics.GetGameInstance`)))
  (`GameplayStatics.PlaySound2D` (`self.Sound`) (* (`/Game/Data/BP_GameInstance.AudioVolume` _asbp_game_instance) 0.01) 1.0 0.0 null null))

(fn `UserConstructionScript`)