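; BP_HurtArea is a damage zone prop that hurts the player while they overlap it.
; Player overlap starts a looping 0.1 second timer, stored in Timer, and ending the overlap clears it.
; Each tick applies a fixed hit through AbsoluteHit on player pawn 0 rather than on the stored overlapping actor.
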(event `self.ReceiveActorBeginOverlap`
  (params (OtherActor :type "Actor Object Reference"))
  (cast `/Game/Player/Blueprints/BP_Player` OtherActor)
  (bind _returnvalue (`KismetSystemLibrary.K2_SetTimerDelegate` (delegate `DamagePlayer`) 0.1 true))
  (set `self.Timer` _returnvalue))

(event `DamagePlayer`
  (bind _asbp_player (cast `/Game/Player/Blueprints/BP_Player` (`GameplayStatics.GetPlayerPawn` 0)))
  (`/Game/Player/Blueprints/BP_Player.AbsoluteHit` _asbp_player 2.0))

(event `self.ReceiveActorEndOverlap`
  (params (OtherActor :type "Actor Object Reference"))
  (cast `/Game/Player/Blueprints/BP_Player` OtherActor)
  (`KismetSystemLibrary.K2_ClearAndInvalidateTimerHandle` (`self.Timer`)))

(fn `UserConstructionScript`)