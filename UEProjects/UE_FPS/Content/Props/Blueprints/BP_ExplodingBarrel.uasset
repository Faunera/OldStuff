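; BP_ExplodingBarrel is a barrel prop that explodes, damaging the player and enemies around it.
; Its Explode event spawns the Niagara effect, then after a short delay queries a sphere component for overlapping actors.
; The overlapping player and each overlapping enemy receive the same fixed damage through their hit functions.
; It then plays a pitched-down grenade sound and destroys itself.
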(event `Explode`
  (bind _sphere (`self.Sphere`))
  (`NiagaraFunctionLibrary.SpawnSystemAtLocation` "/Game/VFX/NS_Explosion.NS_Explosion" (`SceneComponent.K2_GetComponentLocation` (`self.DefaultSceneRoot`)))
  (`KismetSystemLibrary.Delay` 0.4)
  (bind _asbp_player (cast `/Game/Player/Blueprints/BP_Player` (`|GetArrayItem` (`PrimitiveComponent.GetOverlappingActors` _sphere "/Game/Player/Blueprints/BP_Player.BP_Player_C")))
    (:`then`
      (`/Game/Player/Blueprints/BP_Player.OnPlayerHit` _asbp_player 80.0))
    (:`CastFailed`
      _))
  (for _array_element (`PrimitiveComponent.GetOverlappingActors` _sphere "/Game/Enemies/Blueprints/BP_EnemyParent.BP_EnemyParent_C")
    (bind _asbp_enemy_parent (cast `/Game/Enemies/Blueprints/BP_EnemyParent` _array_element))
    (`/Game/Enemies/Blueprints/BP_EnemyParent.OnHit` _asbp_enemy_parent 80.0))
  (`GameplayStatics.PlaySoundAtLocation` "/Game/Audio/Weapons/grenade_explosion.grenade_explosion" (`SceneComponent.K2_GetComponentLocation` (`self.DefaultSceneRoot`)) (struct) 1.0 0.75 0.0 null null null null)
  (`self.K2_DestroyActor`))

(fn `UserConstructionScript`)