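; BP_DoorBig is an interactable double sliding door that opens, then closes itself on a short timer.
; When locked, Interact opens it only if BP_Player's Keys entry at KeyIndex is set; otherwise it calls the parent Interact and opens.
; DoorAnimated plays or reverses one timeline based on DoorClosed, lerping both panels' relative Y positions with sweep.
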(event `self.Interact`
  (if (`self.Locked`)
    (bind _returnvalue (`GameplayStatics.GetActorOfClass` "/Game/Player/Blueprints/BP_Player.BP_Player_C"))
    (if (`|GetArrayItem` (`/Game/Player/Blueprints/BP_Player.Keys` _returnvalue) (`self.KeyIndex`))
      (if (`self.Door closed?`) :!label _label
        (`self.DoorAnimated`)
        (set `self.Door closed?` false)
        (`KismetSystemLibrary.K2_SetTimerDelegate` (delegate `DoorAnimated`) 2.0)))
    (else
      (`parent.Interact`)
      (goto _label))))

(event `DoorAnimated`
  (bind _doorl (`self.DoorL`))
  (bind _doorr (`self.DoorR`))
  (bind (_relativelocation_x _relativelocation_y _relativelocation_z) (`KismetMathLibrary.BreakVector` (`SceneComponent.RelativeLocation` _doorl)))
  (bind (_relativelocation_x_2 _relativelocation_y_2 _relativelocation_z_2) (`KismetMathLibrary.BreakVector` (`SceneComponent.RelativeLocation` _doorr)))
  (if (`self.Door closed?`)
    (bind (_direction _lerp) (`Timeline|Timeline_0` :!via `PlayFromStart` :!label _label_2)
      (:`Update`
        (`SceneComponent.K2_SetRelativeLocation` _doorr (`KismetMathLibrary.MakeVector` _relativelocation_x_2 (`KismetMathLibrary.Lerp` 260.0 0.0 _lerp) _relativelocation_z_2) true false)
        (`SceneComponent.K2_SetRelativeLocation` _doorl (`KismetMathLibrary.MakeVector` _relativelocation_x (`KismetMathLibrary.Lerp` 463.0 697.0 _lerp) _relativelocation_z) true false)))
    (else
      (set `self.Door closed?` true)
      (goto _label_2 :!via `ReverseFromEnd`))))

(fn `UserConstructionScript`)