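; BP_LightB is a light prop Blueprint built around a RectLight component.
; Its construction script applies exposed Color, Height, Width, Intensity and Radius variables to the light's color, source size, brightness and attenuation radius.
; The shown graph contains only this setup, with no runtime logic.
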(fn `UserConstructionScript`
  (bind _rectlight (`self.RectLight`))
  (`LightComponent.SetLightColor` _rectlight (`self.Color`) true)
  (`RectLightComponent.SetSourceHeight` _rectlight (`self.Height`))
  (`RectLightComponent.SetSourceWidth` _rectlight (`self.Width`))
  (`LightComponent.SetIntensity` _rectlight (`self.Intensity`))
  (`LocalLightComponent.SetAttenuationRadius` _rectlight (`self.Radius`)))