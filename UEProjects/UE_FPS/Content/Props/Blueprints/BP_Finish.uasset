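; BP_Finish is the level exit prop that sends the player to the main menu once they hold the required key.
; On overlap it checks the BP_Player's Keys entry at its KeyIndex, then either opens L_MainMenu or shows an escape hint through the player's GameWidget.
; Ending the overlap hides that hint.
; The construction script and DoorAnimated graph are empty.
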(event `self.ReceiveActorBeginOverlap`
  (params (OtherActor :type "Actor Object Reference"))
  (bind _asbp_player (cast `/Game/Player/Blueprints/BP_Player` OtherActor))
  (if (`|GetArrayItem` (`/Game/Player/Blueprints/BP_Player.Keys` _asbp_player) (`self.Key Index`))
    (`GameplayStatics.OpenLevelBySoftObjectPtr` "/Game/Levels/L_MainMenu.L_MainMenu")
    (else
      (`/Game/UI/Blueprints/GameUI/WBP_GameUI.ShowEscapeHint` (`/Game/Player/Blueprints/BP_Player.GameWidget` _asbp_player)))))

(event `self.ReceiveActorEndOverlap`
  (params (OtherActor :type "Actor Object Reference"))
  (bind _asbp_player (cast `/Game/Player/Blueprints/BP_Player` OtherActor))
  (`/Game/UI/Blueprints/GameUI/WBP_GameUI.HideEscapeHint` (`/Game/Player/Blueprints/BP_Player.GameWidget` _asbp_player)))

(fn `DoorAnimated`)

(fn `UserConstructionScript`)