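; BP_DoorSmall01 is an interactable sliding door prop that opens and automatically closes after a short timer.
; When locked, it opens only if BP_Player, found via GetActorOfClass, holds the key at KeyIndex; when unlocked, it calls the parent Interact first.
; DoorAnimated slides the Door along relative X with a swept Timeline lerp, and the timer re-fires it to reverse the Timeline.
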(event `self.Interact`
  (if (`self.Locked`)
    (bind _returnvalue (`GameplayStatics.GetActorOfClass` "/Game/Player/Blueprints/BP_Player.BP_Player_C"))
    (if (`|GetArrayItem` (`/Game/Player/Blueprints/BP_Player.Keys` _returnvalue) (`self.KeyIndex`))
      (if (`self.Door closed?`) :!label _label
        (`self.DoorAnimated`)
        (set `self.Door closed?` false)
        (`KismetSystemLibrary.K2_SetTimerDelegate` (delegate `DoorAnimated`) 2.0)))
    (else
      (`parent.Interact`)
      (goto _label))))

(event `DoorAnimated`
  (bind _door (`self.Door`))
  (bind (_relativelocation_x _relativelocation_y _relativelocation_z) (`KismetMathLibrary.BreakVector` (`SceneComponent.RelativeLocation` _door)))
  (if (`self.Door closed?`)
    (bind (_direction _lerp) (`Timeline|Timeline_0` :!via `PlayFromStart` :!label _label_2)
      (:`Update`
        (`SceneComponent.K2_SetRelativeLocation` _door (`KismetMathLibrary.MakeVector` (`KismetMathLibrary.Lerp` 0.0 -250.0 _lerp) _relativelocation_y _relativelocation_z) true false)))
    (else
      (set `self.Door closed?` true)
      (goto _label_2 :!via `ReverseFromEnd`))))

(fn `UserConstructionScript`)