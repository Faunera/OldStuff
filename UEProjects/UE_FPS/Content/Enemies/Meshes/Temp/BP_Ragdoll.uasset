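; BP_Ragdoll is an enemy ragdoll actor that drops health pickups when it spawns.
; On BeginPlay it enables physics simulation on its skeletal mesh and throws it with a fixed velocity-change impulse.
; It then spawns half-scale BP_HealthPickup actors at random points in a shallow box around its root, with more of them when WasHeadshot is set.
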(event `self.ReceiveBeginPlay`
  (bind _skeletalmesh (`self.SkeletalMesh`))
  (`PrimitiveComponent.SetSimulatePhysics` _skeletalmesh true)
  (`PrimitiveComponent.AddImpulse` _skeletalmesh (0.0 2500.0 -1000.0) "None" true)
  (if (`self.WasHeadshot?`)
    (set `self.OrbIndex` 4)
    (else
      (set `self.OrbIndex` 2)))
  (for _ (range (+ (`self.OrbIndex`) 1))
    (`|SpawnActorFromClass` "/Game/Powerups/BP_HealthPickup.BP_HealthPickup_C" (`KismetMathLibrary.MakeTransform` (`KismetMathLibrary.RandomPointInBoundingBox` (`SceneComponent.K2_GetComponentLocation` (`self.DefaultSceneRoot`)) (100.0 100.0 25.0)) (struct) (0.5 0.5 0.5)) "Undefined" "OverrideRootScale" null null)))

(fn `UserConstructionScript`)