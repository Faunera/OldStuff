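; BP_HealthOrb is a health pickup that homes in on the player and restores health on contact.
; A looping timer started at BeginPlay moves the orb toward the player within a fixed radius, using AttractSpeed.
; Overlapping HealSphere adds RestoreAmount when health is below maximum, which can overshoot it, or otherwise sets health to maximum.
; Either way, the orb plays a pickup sound and destroys itself.
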(event `self.HealSphere.OnComponentBeginOverlap`
  (params (OverlappedComponent :type "PrimitiveComponent Object Reference") (OtherActor :type "Actor Object Reference") (OtherComp :type "PrimitiveComponent Object Reference") (OtherBodyIndex :type Integer) (bFromSweep :type Boolean) (SweepResult :type "HitResult Structure (by ref)"))
  (bind _asbp_player (cast `/Game/Player/Blueprints/BP_Player` OtherActor))
  (bind _health (`/Game/Player/Blueprints/BP_Player.Health` _asbp_player))
  (bind _maxhealth (`/Game/Player/Blueprints/BP_Player.MaxHealth` _asbp_player))
  (if (< _health _maxhealth)
    (set `/Game/Player/Blueprints/BP_Player.Health` (+ _health (`self.RestoreAmount`)) _asbp_player)
    (else
      (set `/Game/Player/Blueprints/BP_Player.Health` _maxhealth _asbp_player)))
  (`GameplayStatics.PlaySoundAtLocation` "/Game/Audio/health_pickup.health_pickup" (`SceneComponent.K2_GetComponentLocation` (`self.HealSphere`)) (struct) 1.0 1.0 0.0 null null null null)
  (`self.K2_DestroyActor`))

(event `self.ReceiveBeginPlay`
  (set `self.Player` (`GameplayStatics.GetPlayerCharacter` 0))
  (`KismetSystemLibrary.K2_SetTimerDelegate` (delegate `PullToPlayer`) 0.01 true))

(event `PullToPlayer`
  (bind _player (`self.Player`))
  (`/Engine/EditorBlueprintResources/StandardMacros.IsValid` _player
    (:`Is Valid`
      (if (<= (`self.GetDistanceTo` _player) 500.0)
        (`self.K2_AddActorWorldOffset` (* (`KismetMathLibrary.Normal` (- (`self.K2_GetActorLocation` _player) (`self.K2_GetActorLocation`))) (`GameplayStatics.GetWorldDeltaSeconds`) (`self.AttractSpeed`)))))))

(fn `UserConstructionScript`)