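; BP_EnemyParent is a base enemy character that spawns and carries a weapon, takes damage and is replaced by a ragdoll on death.
; BeginPlay attaches the weapon with ample ammo and starts a looping timer that re-snaps it to the socket and polls health for death.
; Events handle crouching, randomized-spread firing with reload, melee, and hits that trigger the player's hit indicator and report damage.
; Helpers set walk speed and trace within a narrow cone toward the player.
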(event `self.ReceiveBeginPlay`
  (`KismetSystemLibrary.K2_SetTimerDelegate` (delegate `SetWeaponLocation`) 0.1 true)
  (bind _returnvalue (`|SpawnActorFromClass` (`self.WeaponClassReference`) (`KismetMathLibrary.MakeTransform` (0.0 0.0 0.0) (struct) (0.3 0.3 0.3)) "AlwaysSpawn" "OverrideRootScale" null null))
  (bind _output_get (set `self.WeaponReference` _returnvalue))
  (set `/Game/Weapons/Blueprints/Parents/BP_ParentWeapon.PickedUp` true _output_get)
  (`self.K2_AttachToActor` _output_get self "Grip" "SnapToTarget" "SnapToTarget" "KeepWorld" true)
  (set `/Game/Weapons/Blueprints/Parents/BP_ParentWeapon.TotalAmmo` 10000 (`self.WeaponReference`))
  (bind _weaponreference (`self.WeaponReference`)
    (:`then`
      (set `/Game/Weapons/Blueprints/Parents/BP_ParentWeapon.RateOfFire` (* (`/Game/Weapons/Blueprints/Parents/BP_ParentWeapon.RateOfFire` _weaponreference) 0.5) _weaponreference))
    (:`else`)))

(event `SetWeaponLocation`
  ;[0.04167 0.04167 0.04167] Timer Functions
  (`SceneComponent.K2_SetWorldLocation` (`/Game/Weapons/Blueprints/Parents/BP_ParentWeapon.DefaultSceneRoot` (`self.WeaponReference`)) (`SceneComponent.K2_GetComponentLocation` (`self.WeaponSocket`)) false false)
  (if (<= (`self.Health`) 0.0)
    (`self.Die`)))

(event `Crouch in cover`
  (`self.Crouch`)
  (`KismetSystemLibrary.PrintString` "Enemy crouched" true true (struct :`R` 1.0 :`B` 0.897106 :`A` 1.0)))

(event `Fire`
  (bind _weaponreference (`self.WeaponReference`)
    (:`then`
      (set `/Game/Weapons/Blueprints/Parents/BP_ParentWeapon.Spread` (`KismetMathLibrary.RandomFloatInRange` 0.0 25.0) _weaponreference)
      (`/Game/Weapons/Blueprints/Parents/BP_ParentWeapon.FireWeapon` _weaponreference)
      (if (<= (`/Game/Weapons/Blueprints/Parents/BP_ParentWeapon.CurrentAmmo` _weaponreference) 0)
        (`/Game/Weapons/Blueprints/Parents/BP_ParentWeapon.Reload` (`self.WeaponReference`))))
    (:`else`)))

(event `Melee`
  (bind _asbp_parent_melee (cast `/Game/Weapons/Blueprints/Parents/BP_ParentMelee` (`self.WeaponReference`)))
  (`/Game/Weapons/Blueprints/Parents/BP_ParentWeapon.FireWeapon` _asbp_parent_melee))

(event `OnHit`
  (params (Damage :type "Float (double-precision)"))
  (bind _returnvalue (`GameplayStatics.GetPlayerPawn` 0))
  (bind _asbp_player (cast `/Game/Player/Blueprints/BP_Player` _returnvalue)
    (:`then`
      (`/Game/Player/Blueprints/BP_Player.HitIndicatorEvent` _asbp_player Damage)
      (`AISense_Damage.ReportDamageEvent` self _returnvalue Damage))
    (:`CastFailed`
      _))
  (set `self.Health` (- (`self.Health`) Damage)))

(event `Die`
  (bind _returnvalue (`|SpawnActorFromClass` "/Game/Enemies/Meshes/Temp/BP_Ragdoll.BP_Ragdoll_C" (`SceneComponent.K2_GetComponentToWorld` (`self.CapsuleComponent`)) "AlwaysSpawn" "OverrideRootScale" null null))
  (set `/Game/Enemies/Meshes/Temp/BP_Ragdoll.WasHeadshot?` (>= 0.0 40.0) _returnvalue)
  (`self.K2_DestroyActor` (`self.WeaponReference`))
  (`self.K2_DestroyActor` self))

(fn `Raycast`
  (returns (HitActor :type "Actor Object Reference"))
  (locals (Objects :type "Array of EObjectTypeQuery Enum"))
  (bind _returnvalue (`self.K2_GetActorLocation`))
  (bind _outhit (`KismetSystemLibrary.LineTraceSingleForObjects` :`Start` _returnvalue :`End` (+ _returnvalue (* (`KismetMathLibrary.RandomUnitVectorInConeInDegrees` (`KismetMathLibrary.GetForwardVector` (`KismetMathLibrary.FindLookAtRotation` (`self.K2_GetActorLocation`) (`self.K2_GetActorLocation` (`GameplayStatics.GetPlayerPawn` 0)))) 5.0) 3000.0)) :`ObjectTypes` (`local.Objects`) :`DrawDebugType` "ForDuration"))
  (return (`.HitActor` (`GameplayStatics.BreakHitResult` _outhit))))

(fn `Update Walk Speed`
  (params (NewWalkSpeed :type "Float (double-precision)"))
  (set `CharacterMovementComponent.MaxWalkSpeed` NewWalkSpeed (`self.CharacterMovement`)))

(fn `UserConstructionScript`)