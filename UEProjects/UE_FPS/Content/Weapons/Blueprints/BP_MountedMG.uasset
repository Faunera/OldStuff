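; BP_MountedMG is a mounted machine gun that the player can take control of and release, built on a parent weapon class.
; ControlWeapon swaps input from IMC_Default to IMC_Mounted, halts player movement and attaches the gun to BP_Player.
; DropControl restores default input, detaches the gun and returns it to the transform saved at BeginPlay.
; Raycast defers to the parent, while camera-following rotation and its timer are unwired.
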(event `self.ReceiveBeginPlay`
  (`parent.ReceiveBeginPlay`)
  (set `self.OriginalLocation` (`SceneComponent.K2_GetComponentToWorld` (`self.DefaultSceneRoot`))))

(event `self.Control Weapon`
  (bind _returnvalue (pcsubsystem `EnhancedInputLocalPlayerSubsystem` (`GameplayStatics.GetPlayerController` 0)))
  (`self.Rotate`)
  (`EnhancedInputSubsystemInterface.AddMappingContext` _returnvalue "/Game/Player/Input/IMC_Mounted.IMC_Mounted" 0 (struct))
  (`EnhancedInputSubsystemInterface.RemoveMappingContext` _returnvalue "/Game/Player/Input/IMC_Default.IMC_Default" (struct))
  (bind _asbp_player (cast `/Game/Player/Blueprints/BP_Player` (`GameplayStatics.GetPlayerPawn` 0)))
  (`MovementComponent.StopMovementImmediately` (`Character.CharacterMovement` _asbp_player))
  (`self.K2_AttachToActor` _asbp_player "None" "KeepWorld" "KeepWorld" "KeepWorld" false))

(event `Rotate`
  (bind _staticmesh (`self.StaticMesh`))
  (bind _asbp_player (cast `/Game/Player/Blueprints/BP_Player` (`GameplayStatics.GetPlayerPawn` 0)))
  (`SceneComponent.K2_SetWorldLocation` _staticmesh (`SceneComponent.K2_GetComponentLocation` _staticmesh) false false))

(event `self.Drop Control`
  (bind _returnvalue (pcsubsystem `EnhancedInputLocalPlayerSubsystem` (`GameplayStatics.GetPlayerController` 0)))
  (`EnhancedInputSubsystemInterface.AddMappingContext` _returnvalue "/Game/Player/Input/IMC_Default.IMC_Default" 0 (struct))
  (`EnhancedInputSubsystemInterface.RemoveMappingContext` _returnvalue "/Game/Player/Input/IMC_Mounted.IMC_Mounted" (struct))
  (`self.K2_DetachFromActor` "KeepWorld" "KeepWorld" "KeepWorld")
  (`SceneComponent.K2_SetWorldTransform` (`self.DefaultSceneRoot`) (`self.OriginalLocation`) false false))

(fn `Raycast`
  (params (Range :type "IntVector Structure") (`Spread Angle` :type "Float (double-precision)"))
  (returns (`Hit Actor` :type "Actor Object Reference") (`Hit Location` :type "Vector Structure") (HitComponent :type "PrimitiveComponent Object Reference") (TraceEnd :type "Vector Structure"))
  (bind (_hit_actor _hit_location _hitcomponent _traceend) (`parent.Raycast` Range `Spread Angle`))
  (return _hit_actor _hit_location _hitcomponent _traceend))

(fn `UserConstructionScript`
  (`parent.UserConstructionScript`))