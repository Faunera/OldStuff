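; Shotgun weapon Blueprint that extends a parent weapon's firing and raycast, always tracing with its maximum spread.
; Reloading runs on a looping timer that moves one shell at a time from reserve to magazine, and firing pauses it.
; Firing adds a delayed pump sound and conditionally spawns an empty shell.
; When destroyed, it spawns a shotgun ammo actor below itself.
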(event `self.ReceiveDestroyed`
  (`|SpawnActorFromClass` "/Game/Weapons/Blueprints/Ammo/BP_ShotgunAmmo.BP_ShotgunAmmo_C" (`KismetMathLibrary.MakeTransform` (- (`SceneComponent.K2_GetComponentLocation` (`self.DefaultSceneRoot`)) (0.0 0.0 100.0))) "AlwaysSpawn" "OverrideRootScale" null null))

(event `self.FireWeapon`
  (set `self.Reloading` false)
  (`parent.FireWeapon`)
  (`KismetSystemLibrary.K2_PauseTimerHandle` (stale `self.Reload` _returnvalue))
  (`KismetSystemLibrary.K2_SetTimerDelegate` (delegate `PlayShotgunSound`) 0.1)
  (if (== (`self.Firing Delay`) (/ 1.0 (`self.RateOfFire`)))
    (`|SpawnActorFromClass` "/Game/Weapons/Blueprints/Ammo/BP_EmptyShotgunShell.BP_EmptyShotgunShell_C" (`KismetMathLibrary.MakeTransform` (+ (`SceneComponent.K2_GetComponentLocation` (`self.FireSocket`)) (100.0 0.0 0.0))) "Undefined" "OverrideRootScale" null null)))

(event `self.Reload`
  (if (< (`self.CurrentAmmo`) (`self.MagazineSize`))
    (bind _returnvalue (`KismetSystemLibrary.K2_SetTimerDelegate` (delegate `self.ReloadEventTimer`) (`self.ReloadTime`) true))
    (`ActorSequenceComponent.PlaySequence` (`self.ReloadSequence`))
    (`GameplayStatics.PlaySoundAtLocation` (`self.ReloadSound`) (`SceneComponent.K2_GetComponentLocation` (`self.FireSocket`)) (struct) 1.0 1.0 0.0 null null null null)))

(event `PlayShotgunSound`
  (`GameplayStatics.PlaySoundAtLocation` "/Game/Audio/Weapons/shotgun_pump.shotgun_pump" (`SceneComponent.K2_GetComponentLocation` (`self.FireSocket`)) (struct) 1.0 1.0 0.0 null null null null))

(event `self.ReloadEventTimer`
  (if (and (> (`self.TotalAmmo`) 0) (< (`self.CurrentAmmo`) (`self.MagazineSize`)))
    (set `self.TotalAmmo` (- (`self.TotalAmmo`) 1))
    (set `self.CurrentAmmo` (+ (`self.CurrentAmmo`) 1))
    (`GameplayStatics.PlaySound2D` "/Game/Audio/Weapons/pistol_reload.pistol_reload" 0.3 1.0 0.4 null null)
    (else
      (`KismetSystemLibrary.K2_ClearAndInvalidateTimerHandle` (stale `self.Reload` _returnvalue)))))

(fn `Raycast`
  (params (Range :type "IntVector Structure") (`Spread Angle` :type "Float (double-precision)"))
  (returns (`Hit Actor` :type "Actor Object Reference") (`Hit Location` :type "Vector Structure") (HitComponent :type "PrimitiveComponent Object Reference") (TraceEnd :type "Vector Structure"))
  (bind (_hit_actor _hit_location _hitcomponent _traceend) (`parent.Raycast` Range (`self.Max Spread`)))
  (return _hit_actor _hit_location _hitcomponent _traceend))

(fn `UserConstructionScript`
  (`parent.UserConstructionScript`))