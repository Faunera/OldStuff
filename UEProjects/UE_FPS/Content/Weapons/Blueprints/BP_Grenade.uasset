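; BP_Grenade is a grenade weapon that launches projectiles and regains ammo over time.
; FireWeapon runs the parent's fire logic, then, if CanFire allows, spawns a BP_GrenadeProjectile at FireSocket and launches it along the socket's rotation.
; A successful shot starts a looping recharge timer unless a cooldown is already running.
; Recharge counts the cooldown down, adds one ammo per cycle and stops the timer at the two-grenade cap.
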(event `self.ReceiveBeginPlay`
  (`parent.ReceiveBeginPlay`))

(event `self.FireWeapon`
  (if (< (`self.Firing Delay`) 0.0)
    (`parent.FireWeapon`)
    (if (`self.CanFire`)
      (bind _returnvalue (`|SpawnActorFromClass` "/Game/Weapons/Blueprints/BP_GrenadeProjectile.BP_GrenadeProjectile_C" (`KismetMathLibrary.MakeTransform` (`SceneComponent.K2_GetComponentLocation` (`self.FireSocket`))) "Undefined" "OverrideRootScale" null null))
      (`/Engine/EditorBlueprintResources/StandardMacros.IsValid` _returnvalue
        (:`Is Valid`
          (`/Game/Weapons/Blueprints/BP_GrenadeProjectile.LaunchProjectile` _returnvalue (`SceneComponent.K2_GetComponentRotation` (`self.FireSocket`)))
          (if (not (> (`self.Cooldown`) 0.0))
            (set `self.Cooldown` 20.0)
            (bind _returnvalue_2 (`KismetSystemLibrary.K2_SetTimerDelegate` (delegate `Recharge`) 0.1 true))))))))

(event `Recharge`
  (set `self.Cooldown` (- (`self.Cooldown`) 0.1))
  (if (< (`self.Cooldown`) 0.0)
    (bind _output_get (set `self.CurrentAmmo` (+ (`self.CurrentAmmo`) 1)))
    (if (< _output_get 2)
      (set `self.Cooldown` 20.0)
      (else
        (`KismetSystemLibrary.K2_ClearAndInvalidateTimerHandle` (stale `self.FireWeapon` _returnvalue_2))))))

(fn `UserConstructionScript`
  (`parent.UserConstructionScript`))