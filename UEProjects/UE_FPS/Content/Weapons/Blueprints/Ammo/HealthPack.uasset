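; Health pack pickup that heals BP_Player and then destroys itself.
; Both Interact, which uses player pawn 0, and actor overlap route into a shared Pickup event.
; Pickup acts only when Health is below MaxHealth, adding HealAmount through a clamp whose minimum is the healed total itself and whose maximum is MaxHealth.
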(event `self.Interact`
  (bind _asbp_player (cast `/Game/Player/Blueprints/BP_Player` (`GameplayStatics.GetPlayerPawn` 0)))
  (`self.Pickup` _asbp_player))

(event `self.ReceiveActorBeginOverlap`
  (params (OtherActor :type "Actor Object Reference"))
  (bind _asbp_player (cast `/Game/Player/Blueprints/BP_Player` OtherActor))
  (`self.Pickup` _asbp_player))

(event `self.Pickup`
  (params (`Player Reference` :type "/Game/Player/Blueprints/BP_Player Object Reference"))
  (bind _health (`/Game/Player/Blueprints/BP_Player.Health` `Player Reference`))
  (bind _maxhealth (`/Game/Player/Blueprints/BP_Player.MaxHealth` `Player Reference`))
  (bind _returnvalue (+ _health (`self.HealAmount`)))
  (`/Engine/EditorBlueprintResources/StandardMacros.IsValid` `Player Reference`
    (:`Is Valid`
      (if (< _health _maxhealth)
        (set `/Game/Player/Blueprints/BP_Player.Health` (`KismetMathLibrary.FClamp` _returnvalue _returnvalue _maxhealth) `Player Reference`)
        (`self.K2_DestroyActor`)))))

(fn `UserConstructionScript`)