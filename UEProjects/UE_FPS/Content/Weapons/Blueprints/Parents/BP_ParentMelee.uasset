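; BP_ParentMelee is a base melee weapon usable by both player and enemies, built on a parent weapon class.
; A looping timer drives the inherited firing timer logic.
; FireWeapon is gated by FiringDelay, then plays sound and recoil and raycasts over Range without spread.
; The attach parent decides the target: enemy-held weapons damage BP_Player, others damage BP_EnemyParent, while Reload does nothing.
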(event `self.ReceiveBeginPlay`
  (`parent.ReceiveBeginPlay`)
  (`KismetSystemLibrary.K2_SetTimerDelegate` (delegate `self.Firing Timer`) 0.01 true))

(event `self.Firing Timer`
  (`parent.Firing Timer`))

(event `self.ReceiveActorBeginOverlap`
  (params (OtherActor :type "Actor Object Reference"))
  (`parent.ReceiveActorBeginOverlap` OtherActor))

(event `self.FireWeapon`
  (bind _damage (`self.Damage`))
  (if (< (`self.Firing Delay`) 0.0)
    (`GameplayStatics.PlaySound2D` (`self.FireSound`) 1.0 1.0 0.0 null null)
    (set `self.Firing Delay` (/ 1.0 (`self.RateOfFire`)))
    (`ActorSequenceComponent.PlaySequence` (`self.RecoilSequence`))
    (bind _hit_actor (`self.Raycast` (`KismetMathLibrary.Conv_IntToIntVector` (`self.Range`))))
    (cast `/Game/Enemies/Blueprints/BP_EnemyParent` (`self.GetAttachParentActor`)
      (:`then`
        (bind _asbp_player (cast `/Game/Player/Blueprints/BP_Player` _hit_actor))
        (`/Game/Player/Blueprints/BP_Player.OnPlayerHit` _asbp_player _damage)
        (`GameplayStatics.PlaySound2D` "/Game/Audio/Weapons/melee_hit.melee_hit" 1.0 1.0 0.0 null null))
      (:`CastFailed`
        (bind _asbp_enemy_parent (cast `/Game/Enemies/Blueprints/BP_EnemyParent` _hit_actor))
        (`/Game/Enemies/Blueprints/BP_EnemyParent.OnHit` _asbp_enemy_parent _damage)
        (`GameplayStatics.PlaySound2D` "/Game/Audio/Weapons/melee_hit.melee_hit" 1.0 1.0 0.0 null null)
        (`KismetSystemLibrary.PrintString` "Enemy Hit")))))

(event `self.Reload`)

(fn `UserConstructionScript`
  (`parent.UserConstructionScript`))