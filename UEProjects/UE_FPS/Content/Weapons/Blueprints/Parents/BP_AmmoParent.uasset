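; BP_AmmoParent is the parent Blueprint for ammo pickups that refill one of the player's weapons on overlap.
; When a BP_Player overlaps it, it searches the player's WeaponReferences for valid weapons tagged with its WeaponReference value.
; On a match it plays a 2D sound, passes that weapon and its Ammo amount to the player's PickUpAmmo, then destroys itself.
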(event `self.ReceiveActorBeginOverlap`
  (params (OtherActor :type "Actor Object Reference"))
  (bind _asbp_player (cast `/Game/Player/Blueprints/BP_Player` OtherActor))
  (for _array_element (`/Game/Player/Blueprints/BP_Player.Weapon References` _asbp_player)
    (`/Engine/EditorBlueprintResources/StandardMacros.IsValid` _array_element
      (:`Is Valid`
        (if (`self.ActorHasTag` _array_element (`self.Weapon Reference`))
          (`GameplayStatics.PlaySound2D` (`self.Sound`) 1.0 1.0 0.0 null null)
          (`/Game/Player/Blueprints/BP_Player.PickUpAmmo` _asbp_player _array_element (`self.Ammo`))
          (`self.K2_DestroyActor`))))))

(fn `UserConstructionScript`)