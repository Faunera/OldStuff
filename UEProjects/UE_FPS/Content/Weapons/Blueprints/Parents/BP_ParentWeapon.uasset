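; Base weapon Blueprint for players and enemies, handling pickup on player overlap, ammo, firing and timed reloads.
; Fast looping timers count down fire delay, decay spread and snap picked-up weapons to the player's socket.
; FireWeapon sets CanFire, spends ammo and plays recoil and sound; an empty player weapon dry-fires and calls Reload.
; Raycast returns cone-randomized trace hits from the owner's FireOrigin, aiming enemy shots at the player.
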(event `self.ReceiveBeginPlay`
  (`KismetSystemLibrary.K2_SetTimerDelegate` (delegate `Firing Timer`) 0.01 true)
  (`KismetSystemLibrary.K2_SetTimerDelegate` (delegate `RotateWeapon`) 0.001 true))

(event `Firing Timer`
  (bind _spread (`self.Spread`))
  (set `self.Firing Delay` (- (`self.Firing Delay`) 0.01))
  (if (> _spread 0.0)
    (set `self.Spread` (- _spread 0.04))))

(event `RotateWeapon`
  (if (`self.PickedUp`)
    (bind _asbp_player (cast `/Game/Player/Blueprints/BP_Player` (`self.GetAttachParentActor`)))
    (bind _weaponsocket (`/Game/Player/Blueprints/BP_Player.WeaponSocket` _asbp_player))
    (bind (_returnvalue_roll _returnvalue_pitch _returnvalue_yaw) (`KismetMathLibrary.BreakRotator` (`SceneComponent.K2_GetComponentRotation` _weaponsocket)))
    (`self.K2_SetActorRotation` (`KismetMathLibrary.MakeRotator` _returnvalue_roll _returnvalue_pitch (+ _returnvalue_yaw -2.0)))
    (`self.K2_SetActorLocation` (`SceneComponent.K2_GetComponentLocation` _weaponsocket))))

(event `self.ReceiveActorBeginOverlap`
  (params (OtherActor :type "Actor Object Reference"))
  (bind _asbp_player (cast `/Game/Player/Blueprints/BP_Player` OtherActor))
  (if (not (or (`self.ActorHasTag` "Mounted") (`self.PickedUp`)))
    (`SceneComponent.SetWorldScale3D` (`self.DefaultSceneRoot`) (0.25 0.25 0.25))
    (`/Game/Player/Blueprints/BP_Player.Pick Up Weapon` _asbp_player self)))

(event `FireWeapon`
  (if (and (> (`self.CurrentAmmo`) 0) (not (`self.Reloading`)))
    (set `self.CanFire` true)
    (set `self.CurrentAmmo` (- (`self.CurrentAmmo`) 1))
    (set `self.Firing Delay` (/ 1.0 (`self.RateOfFire`)))
    (`ActorSequenceComponent.PlaySequence` (`self.RecoilSequence`))
    (bind _asbp_game_instance (cast `/Game/Data/BP_GameInstance` (`GameplayStatics.GetGameInstance`))
      (:`then`
        (`GameplayStatics.PlaySoundAtLocation` (`self.FireSound`) (`SceneComponent.K2_GetComponentLocation` (`self.FireSocket`)) (struct) (* (`/Game/Data/BP_GameInstance.AudioVolume` _asbp_game_instance) 0.01) 1.0 0.0 null null null null))
      (:`CastFailed`
        (`KismetSystemLibrary.PrintString` "Failed to play weapon sound")))
    (else
      (set `self.CanFire` false)
      (set `self.Firing Delay` (/ 1.0 (`self.RateOfFire`)))
      (bind _asbp_game_instance_2 (cast `/Game/Data/BP_GameInstance` (`GameplayStatics.GetGameInstance`))
        (:`then`
          (cast `/Game/Player/Blueprints/BP_Player` (`self.GetAttachParentActor`))
          (`GameplayStatics.PlaySoundAtLocation` "/Game/Audio/dryfire.dryfire" (`SceneComponent.K2_GetComponentLocation` (`self.FireSocket`)) (struct) (* (`/Game/Data/BP_GameInstance.AudioVolume` _asbp_game_instance_2) 0.01) 1.0 0.0 null null null null)
          (`self.Reload`))
        (:`CastFailed`
          (`KismetSystemLibrary.PrintString` "Failed to play weapon sound"))))))

(event `Reload`
  (if (and (< (`self.CurrentAmmo`) (`self.MagazineSize`)) (not (`self.Reloading`)) (> (`self.TotalAmmo`) 0))
    (set `self.Reloading` true)
    (`KismetSystemLibrary.K2_SetTimerDelegate` (delegate `ReloadEventTimer`) (`self.ReloadTime`))
    (`ActorSequenceComponent.PlaySequence` (`self.ReloadSequence`))
    (bind _asbp_game_instance (cast `/Game/Data/BP_GameInstance` (`GameplayStatics.GetGameInstance`))
      (:`then`
        (`GameplayStatics.PlaySoundAtLocation` (`self.ReloadSound`) (`SceneComponent.K2_GetComponentLocation` (`self.FireSocket`)) (struct) (* (`/Game/Data/BP_GameInstance.AudioVolume` _asbp_game_instance) 0.01) 1.0 0.0 null null null null))
      (:`CastFailed`
        (`KismetSystemLibrary.PrintString` "Failed to play weapon sound")))))

(event `ReloadEventTimer`
  (bind _magazinesize (`self.MagazineSize`))
  (bind _returnvalue (- (`self.TotalAmmo`) (- _magazinesize (`self.CurrentAmmo`))))
  (set `self.Reloading` false)
  (if (> _returnvalue 0)
    (set `self.TotalAmmo` _returnvalue)
    (set `self.CurrentAmmo` _magazinesize)
    (else
      (set `self.CurrentAmmo` (+ (`self.TotalAmmo`) (`self.CurrentAmmo`)))
      (set `self.TotalAmmo` 0))))

(event `Add Ammo`
  (params (`Ammo amount` :type Integer))
  (set `self.TotalAmmo` (+ (`self.TotalAmmo`) `Ammo amount`)))

(event `Control Weapon`)

(event `Drop Control`)

(fn `Raycast`
  (params (Range :type "IntVector Structure") (`Spread Angle` :type "Float (double-precision)"))
  (returns (`Hit Actor` :type "Actor Object Reference") (`Hit Location` :type "Vector Structure") (HitComponent :type "PrimitiveComponent Object Reference") (TraceEnd :type "Vector Structure"))
  (bind _returnvalue (`self.GetAttachParentActor`))
  (bind _array (`|MakeArray` (`self.GetAttachParentActor`) null))
  (bind _asbp_player (cast `/Game/Player/Blueprints/BP_Player` _returnvalue)
    (:`then`
      (bind _fireorigin (`/Game/Player/Blueprints/BP_Player.FireOrigin` _asbp_player))
      (bind _returnvalue_2 (`SceneComponent.K2_GetComponentLocation` _fireorigin))
      (bind _outhit (`KismetSystemLibrary.LineTraceSingleForObjects` _returnvalue_2 (+ _returnvalue_2 (* (`KismetMathLibrary.RandomUnitVectorInConeInDegrees` (`KismetMathLibrary.GetForwardVector` (`SceneComponent.K2_GetComponentRotation` _fireorigin)) `Spread Angle`) Range)) (`self.Object Types`) false _array))
      (bind (_bblockinghit _binitialoverlap _time _distance _location _impactpoint _normal _impactnormal _physmat _hitactor _hitcomponent _hitbonename _bonename _hititem _elementindex _faceindex _tracestart _traceend) (`GameplayStatics.BreakHitResult` _outhit))
      (return _hitactor _impactpoint _hitcomponent _traceend))
    (:`CastFailed`
      (bind _asbp_enemy_parent (cast `/Game/Enemies/Blueprints/BP_EnemyParent` _returnvalue))
      (bind _returnvalue_3 (`SceneComponent.K2_GetComponentLocation` (`/Game/Enemies/Blueprints/BP_EnemyParent.FireOrigin` _asbp_enemy_parent)))
      (bind _outhit_2 (`KismetSystemLibrary.LineTraceSingleForObjects` _returnvalue_3 (+ _returnvalue_3 (* (`KismetMathLibrary.RandomUnitVectorInConeInDegrees` (`KismetMathLibrary.GetForwardVector` (`KismetMathLibrary.FindLookAtRotation` _returnvalue_3 (`self.K2_GetActorLocation` (`GameplayStatics.GetPlayerPawn` 0)))) `Spread Angle`) Range)) (`self.Object Types`) false _array))
      (bind (_bblockinghit_2 _binitialoverlap_2 _time_2 _distance_2 _location_2 _impactpoint_2 _normal_2 _impactnormal_2 _physmat_2 _hitactor_2 _hitcomponent_2 _hitbonename_2 _bonename_2 _hititem_2 _elementindex_2 _faceindex_2 _tracestart_2 _traceend_2) (`GameplayStatics.BreakHitResult` _outhit_2))
      (return _hitactor_2 _impactpoint_2 _hitcomponent_2 _traceend_2))))

(fn `UserConstructionScript`)