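; BP_ParentProjectile is a parent weapon Blueprint, named for projectile weapons, that extends an inherited firing and raycast base.
; FireWeapon calls the parent only when FiringDelay is below zero, then checks CanFire with nothing wired after it, so no projectile spawns here.
; The Raycast override forces zero spread on the parent trace, passes through hit actor and location, and returns a zero TraceEnd.
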(event `self.FireWeapon`
  (if (< (`self.Firing Delay`) 0.0)
    (`parent.FireWeapon`)
    (if (`self.CanFire`)
      _)))

(fn `Raycast`
  (params (Range :type "IntVector Structure") (`Spread Angle` :type "Float (double-precision)"))
  (returns (`Hit Actor` :type "Actor Object Reference") (`Hit Location` :type "Vector Structure") (HitComponent :type "PrimitiveComponent Object Reference") (TraceEnd :type "Vector Structure"))
  (bind (_hit_actor _hit_location) (`parent.Raycast` Range 0.0))
  (return _hit_actor _hit_location null (0.0 0.0 0.0)))

(fn `UserConstructionScript`
  (`parent.UserConstructionScript`))