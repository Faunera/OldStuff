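; Grenade projectile that travels along its own spline and deals area damage to enemies when it explodes.
; LaunchProjectile orients the spline and starts a fast looping timer that sweeps the sphere along it by accumulated distance.
; Non-player hits or InnerArea overlaps, the spline's end or an accumulated-time limit trigger the explosion.
; Explosion damages enemies in AreaEffect, doubling it for capsules within an inner radius, then destroys the actor.
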(event `LaunchProjectile`
  (params (Rotation :type "Rotator Structure"))
  (`SceneComponent.K2_SetWorldRotation` (`self.Spline`) Rotation false false)
  (`KismetSystemLibrary.K2_SetTimerDelegate` (delegate `MoveAlongSpline`) 0.001 true))

(event `MoveAlongSpline`
  (bind _spline (`self.Spline`))
  (set `self.Timer` (+ (`self.Timer`) 0.001))
  (set `self.Distance` (+ (* (`self.Speed`) 0.1) (`self.Distance`)))
  (`SceneComponent.K2_SetWorldLocation` (`self.Sphere`) (`SplineComponent.GetLocationAtDistanceAlongSpline` (`self.Spline`) (`self.Distance`) "World") true false)
  (`/Engine/EditorBlueprintResources/StandardMacros.IsValid` _spline
    (:`Is Valid`
      (if (or (>= (`self.Distance`) (`SplineComponent.GetSplineLength` _spline)) (> (`self.Timer`) 3.0))
        (`self.Explosion`)))))

(event `self.Sphere.OnComponentHit`
  (params (HitComponent :type "PrimitiveComponent Object Reference") (OtherActor :type "Actor Object Reference") (OtherComp :type "PrimitiveComponent Object Reference") (NormalImpulse :type "Vector Structure") (Hit :type "HitResult Structure (by ref)"))
  (cast `/Game/Player/Blueprints/BP_Player` OtherActor
    (:`CastFailed`
      (`self.Explosion`))))

(event `self.InnerArea.OnComponentBeginOverlap`
  (params (OverlappedComponent :type "PrimitiveComponent Object Reference") (OtherActor :type "Actor Object Reference") (OtherComp :type "PrimitiveComponent Object Reference") (OtherBodyIndex :type Integer) (bFromSweep :type Boolean) (SweepResult :type "HitResult Structure (by ref)"))
  (cast `/Game/Player/Blueprints/BP_Player` OtherActor
    (:`CastFailed`
      (`self.Explosion`))))

(event `Explosion`
  (bind _damage (`self.Damage`))
  (`GameplayStatics.PlaySound2D` "/Game/Audio/Weapons/grenade_explosion.grenade_explosion" 0.2 1.0 0.0 null null)
  (for _array_element (`PrimitiveComponent.GetOverlappingActors` (`self.AreaEffect`) "/Game/Enemies/Blueprints/BP_EnemyParent.BP_EnemyParent_C")
    (bind _asbp_enemy_parent (cast `/Game/Enemies/Blueprints/BP_EnemyParent` _array_element))
    (bind (_hitlocation _hitnormal _bonename _outhit _returnvalue) (`PrimitiveComponent.K2_SphereOverlapComponent` (`Character.CapsuleComponent` _asbp_enemy_parent) (`SceneComponent.K2_GetComponentLocation` (`self.Sphere`)) 150.0 false false false))
    (if _returnvalue
      (`KismetSystemLibrary.PrintString` "Hello")
      (`/Game/Enemies/Blueprints/BP_EnemyParent.OnHit` _asbp_enemy_parent (* _damage 2.0))
      (else
        (`KismetSystemLibrary.PrintString` "uwu")
        (`/Game/Enemies/Blueprints/BP_EnemyParent.OnHit` _asbp_enemy_parent _damage)))
    (`KismetSystemLibrary.PrintString` "Enemy Hit with explosion"))
  (`KismetSystemLibrary.PrintString` "Grenade done")
  (`self.K2_DestroyActor`))

(fn `UserConstructionScript`)