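; BP_Pistol is a pistol weapon actor that leaves a pistol ammo actor behind when it is destroyed.
; Its Destroyed event spawns BP_PistolAmmo at a fixed offset below the scene root's world location, ignoring collisions.
; The other events are disabled stubs and the construction script only calls the parent, so the graphs hold no firing or pickup logic.
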(event `self.ReceiveDestroyed`
  (`|SpawnActorFromClass` "/Game/Weapons/Blueprints/Ammo/BP_PistolAmmo.BP_PistolAmmo_C" (`KismetMathLibrary.MakeTransform` (- (`SceneComponent.K2_GetComponentLocation` (`self.DefaultSceneRoot`)) (0.0 0.0 100.0))) "AlwaysSpawn" "OverrideRootScale" null null))

(fn `UserConstructionScript`
  (`parent.UserConstructionScript`))