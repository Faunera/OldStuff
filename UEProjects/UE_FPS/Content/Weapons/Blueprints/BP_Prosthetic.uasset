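; BP_Prosthetic is a weapon Blueprint that can smash destructible objects, built on a parent that supplies pickup and firing behavior.
; On overlap it runs the parent logic, then plays a major pickup sound if not yet picked up.
; When the firing delay has expired, firing calls the parent, then raycasts without spread over the weapon's range and calls Smashed on any BP_Destructible hit.
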(event `self.ReceiveActorBeginOverlap`
  (params (OtherActor :type "Actor Object Reference"))
  (`parent.ReceiveActorBeginOverlap` OtherActor)
  (if (not (`self.PickedUp`))
    (`GameplayStatics.PlaySound2D` "/Game/Audio/major_pickup.major_pickup" 1.0 1.0 0.0 null null)))

(event `self.FireWeapon`
  (if (<= (`self.Firing Delay`) 0.0)
    (`parent.FireWeapon`)
    (bind _hit_actor (`self.Raycast` (`KismetMathLibrary.Conv_IntToIntVector` (`self.Range`))))
    (bind _asbp_destructible (cast `/Game/Props/Blueprints/BP_Destructible` _hit_actor))
    (`/Game/Props/Blueprints/BP_Destructible.Smashed` _asbp_destructible)))

(fn `UserConstructionScript`
  (`parent.UserConstructionScript`))