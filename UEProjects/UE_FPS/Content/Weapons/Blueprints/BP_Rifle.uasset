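; Rifle weapon Blueprint that adds firing and reload visuals on top of its parent weapon logic.
; Firing calls the parent, then plays a sped-up fire animation if ammo remains and none is playing.
; Reloading swaps the skeletal mesh to SM_Vulture_Rifle, and a ReloadTime timer switches it to Vulture.
; When destroyed, it spawns a BP_RifleAmmo actor just below its root location.
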(event `self.ReceiveDestroyed`
  (`|SpawnActorFromClass` "/Game/Weapons/Blueprints/Ammo/BP_RifleAmmo.BP_RifleAmmo_C" (`KismetMathLibrary.MakeTransform` (- (`SceneComponent.K2_GetComponentLocation` (`self.DefaultSceneRoot`)) (0.0 0.0 100.0))) "AlwaysSpawn" "OverrideRootScale" null null))

(event `self.FireWeapon`
  (bind _skeletalmesh (`self.SkeletalMesh`))
  (`parent.FireWeapon`)
  (if (> (`self.CurrentAmmo`) 0)
    (if (not (`SkeletalMeshComponent.IsPlaying` _skeletalmesh))
      (`SkeletalMeshComponent.PlayAnimation` _skeletalmesh "/Game/Weapons/Animations/RifleFire.RifleFire" false)
      (`SkeletalMeshComponent.SetPlayRate` _skeletalmesh 2.0))))

(event `self.Reload`
  (`parent.Reload`)
  (`KismetSystemLibrary.K2_SetTimerDelegate` (delegate `ChangeSkeleton`) (`self.ReloadTime`))
  (`SkeletalMeshComponent.SetSkeletalMeshAsset` (`self.SkeletalMesh`) "/Game/Weapons/Meshes/SM_Vulture_Rifle.SM_Vulture_Rifle"))

(event `ChangeSkeleton`
  (`SkeletalMeshComponent.SetSkeletalMeshAsset` (`self.SkeletalMesh`) "/Game/Weapons/Meshes/Vulture.Vulture"))

(fn `UserConstructionScript`
  (`parent.UserConstructionScript`))