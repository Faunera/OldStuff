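; Movement buff pickup that raises the player's walk and crouched walk speeds on overlap.
; When BP_Player touches it, it calls SaveBuff, then plays a 2D pickup sound scaled by the GameInstance audio volume.
; It then adds fixed amounts to both CharacterMovement speeds, prints debug text and destroys itself.
; The increase has no timer or revert in this Blueprint, and BeginPlay only calls the parent.
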(event `self.ReceiveBeginPlay`
  (`parent.ReceiveBeginPlay`))

(event `self.ReceiveActorBeginOverlap`
  (params (OtherActor :type "Actor Object Reference"))
  (bind _asbp_player (cast `/Game/Player/Blueprints/BP_Player` OtherActor))
  (`self.Save Buff`)
  (bind _asbp_game_instance (cast `/Game/Data/BP_GameInstance` (`GameplayStatics.GetGameInstance`)))
  (`GameplayStatics.PlaySound2D` "/Game/Audio/major_pickup.major_pickup" (* (`/Game/Data/BP_GameInstance.AudioVolume` _asbp_game_instance) 0.01) 1.0 0.0 null null)
  (bind _charactermovement (`Character.CharacterMovement` _asbp_player))
  (bind _output_get (set `CharacterMovementComponent.MaxWalkSpeed` (+ (`CharacterMovementComponent.MaxWalkSpeed` _charactermovement) 70.0) _charactermovement))
  (set `CharacterMovementComponent.MaxWalkSpeedCrouched` (+ (`CharacterMovementComponent.MaxWalkSpeedCrouched` _charactermovement) 50.0) _charactermovement)
  (`KismetSystemLibrary.PrintString` "Picked up movement buff")
  (`KismetSystemLibrary.PrintString` (`KismetStringLibrary.Conv_DoubleToString` _output_get))
  (`self.K2_DestroyActor`))

(fn `UserConstructionScript`)