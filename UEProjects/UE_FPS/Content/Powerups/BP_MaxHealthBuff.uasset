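; BP_MaxHealthBuff is a pickup that permanently raises the player's max health and refills health to full.
; A looping timer spins its static mesh while it waits in the level.
; On overlap with BP_Player it calls SaveBuff, plays a pickup sound scaled by the game instance's audio volume, applies the buff, spawns a Niagara effect and destroys itself.
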(event `self.ReceiveBeginPlay`
  (`parent.ReceiveBeginPlay`)
  (`KismetSystemLibrary.K2_SetTimerDelegate` (delegate `Rotation`) 0.01 true))

(event `Rotation`
  (`SceneComponent.K2_AddLocalRotation` (`self.StaticMesh`) (struct :`Yaw` -2.0) false false))

(event `self.ReceiveActorBeginOverlap`
  (params (OtherActor :type "Actor Object Reference"))
  (bind _asbp_player (cast `/Game/Player/Blueprints/BP_Player` OtherActor))
  (`self.Save Buff`)
  (bind _asbp_game_instance (cast `/Game/Data/BP_GameInstance` (`GameplayStatics.GetGameInstance`))
    (:`then`
      (`GameplayStatics.PlaySound2D` "/Game/Audio/major_pickup.major_pickup" (* (`/Game/Data/BP_GameInstance.AudioVolume` _asbp_game_instance) 0.01) 1.0 0.0 null null))
    (:`CastFailed`
      _))
  (bind _output_get (set `/Game/Player/Blueprints/BP_Player.MaxHealth` (+ (`/Game/Player/Blueprints/BP_Player.MaxHealth` _asbp_player) 10.0) _asbp_player))
  (set `/Game/Player/Blueprints/BP_Player.Health` _output_get _asbp_player)
  (`NiagaraFunctionLibrary.SpawnSystemAtLocation` "/Game/VFX/NS_HealthUpgrade.NS_HealthUpgrade" (`SceneComponent.K2_GetComponentLocation` (`self.StaticMesh`)))
  (`self.K2_DestroyActor`))

(fn `UserConstructionScript`)