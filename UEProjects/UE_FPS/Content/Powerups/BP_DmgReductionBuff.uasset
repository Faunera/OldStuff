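; BP_DmgReductionBuff is a pickup that permanently adds to the player's DamageReduction stat on overlap.
; A looping timer spins its Sphere component in small steps.
; When BP_Player overlaps, it calls SaveBuff (not defined in this file), plays a pickup sound scaled by the GameInstance audio volume, raises the stat and destroys itself.
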(event `self.ReceiveBeginPlay`
  (`parent.ReceiveBeginPlay`)
  (`KismetSystemLibrary.K2_SetTimerDelegate` (delegate `Spin`) 0.1 true))

(event `Spin`
  (`SceneComponent.K2_AddLocalRotation` (`self.Sphere`) (struct :`Yaw` 0.1 :`Roll` 0.1) false false))

(event `self.ReceiveActorBeginOverlap`
  (params (OtherActor :type "Actor Object Reference"))
  (bind _asbp_player (cast `/Game/Player/Blueprints/BP_Player` OtherActor))
  (`self.Save Buff`)
  (bind _asbp_game_instance (cast `/Game/Data/BP_GameInstance` (`GameplayStatics.GetGameInstance`))
    (:`then`
      (`GameplayStatics.PlaySound2D` "/Game/Audio/major_pickup.major_pickup" (* (`/Game/Data/BP_GameInstance.AudioVolume` _asbp_game_instance) 0.01) 1.0 0.0 null null))
    (:`CastFailed`
      _))
  (set `/Game/Player/Blueprints/BP_Player.DamageReduction` (+ (`/Game/Player/Blueprints/BP_Player.DamageReduction` _asbp_player) 2.0) _asbp_player)
  (`self.K2_DestroyActor`))

(fn `UserConstructionScript`)