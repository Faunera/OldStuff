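; BP_Jetpack is a jetpack pickup that registers itself on BP_Player on overlap, if none is held, and hides its mesh.
; Each UseJetpack call pauses recharging, spends charge, applies an upward impulse to player 0 and plays thrust audio scaled by the game instance's volume.
; Stopping starts a looping timer that refills charge to its cap; stopping or running empty also sets Falling movement and cuts the audio.
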(event `Use Jetpack`
  (bind _audio (`self.Audio`))
  (bind _charactermovement (`Character.CharacterMovement` (`GameplayStatics.GetPlayerCharacter` 0)))
  (`KismetSystemLibrary.K2_PauseTimerHandle` (stale `Stop Jetpack` _returnvalue))
  (if (>= (`self.JetpackCharge`) 1.0)
    (set `self.JetpackCharge` (- (`self.JetpackCharge`) 0.5))
    (`CharacterMovementComponent.AddImpulse` _charactermovement (0.0 0.0 1500.0) false)
    (if (not (`AudioComponent.IsPlaying` _audio))
      (bind _asbp_game_instance (cast `/Game/Data/BP_GameInstance` (`GameplayStatics.GetGameInstance`)))
      (`AudioComponent.SetVolumeMultiplier` _audio (* (* (`/Game/Data/BP_GameInstance.AudioVolume` _asbp_game_instance) 0.01) 0.5))
      (`AudioComponent.Play` _audio 0.0))
    (else
      (`CharacterMovementComponent.SetMovementMode` _charactermovement "MOVE_Falling" 0 :!label _label)
      (`AudioComponent.StopDelayed` (`self.Audio`) 0.1))))

(event `Stop Jetpack`
  (bind _returnvalue (`KismetSystemLibrary.K2_SetTimerDelegate` (delegate `ChargeJetpack`) 0.1 true))
  (goto _label))

(event `ChargeJetpack`
  (if (>= (`self.JetpackCharge`) 100.0)
    (`KismetSystemLibrary.K2_ClearAndInvalidateTimerHandle` (stale `Stop Jetpack` _returnvalue))
    (else
      (set `self.JetpackCharge` (+ (`self.JetpackCharge`) 2.0)))))

(event `self.ReceiveActorBeginOverlap`
  (params (OtherActor :type "Actor Object Reference"))
  (bind _asbp_player (cast `/Game/Player/Blueprints/BP_Player` OtherActor))
  (`/Engine/EditorBlueprintResources/StandardMacros.IsValid` (`/Game/Player/Blueprints/BP_Player.Jetpack` _asbp_player)
    (:`Is Valid`
      _)
    (:`Is Not Valid`
      (set `/Game/Player/Blueprints/BP_Player.Jetpack` self _asbp_player)
      (`GameplayStatics.PlaySound2D` "/Game/Audio/major_pickup.major_pickup" 1.0 1.0 0.0 null null)))
  (`SceneComponent.SetVisibility` (`self.StaticMesh`) false false))

(fn `UserConstructionScript`)