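; BP_InfiniteAmmo is a powerup pickup that gives the player effectively infinite ammo.
; On overlap with BP_Player, it plays a pickup sound scaled by the GameInstance audio volume and sets CurrentAmmo on every entry in the player's WeaponReferences to a very large fixed value.
; It then prints a debug message and destroys itself; there is no timer, so the refill is a one-time set rather than a true unlimited-ammo state.
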(event `self.ReceiveActorBeginOverlap`
  (params (OtherActor :type "Actor Object Reference"))
  (bind _asbp_player (cast `/Game/Player/Blueprints/BP_Player` OtherActor))
  (bind _asbp_game_instance (cast `/Game/Data/BP_GameInstance` (`GameplayStatics.GetGameInstance`))
    (:`then`
      (`GameplayStatics.PlaySound2D` "/Game/Audio/major_pickup.major_pickup" (* (`/Game/Data/BP_GameInstance.AudioVolume` _asbp_game_instance) 0.01) 1.0 0.0 null null))
    (:`CastFailed`
      _))
  (for _array_element (`/Game/Player/Blueprints/BP_Player.Weapon References` _asbp_player)
    (set `/Game/Weapons/Blueprints/Parents/BP_ParentWeapon.CurrentAmmo` 10000 _array_element))
  (`KismetSystemLibrary.PrintString` "Picked infinite ammo")
  (`self.K2_DestroyActor`))

(fn `UserConstructionScript`)