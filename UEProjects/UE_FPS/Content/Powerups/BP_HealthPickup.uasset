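; BP_HealthPickup is a powerup that restores the player's health on overlap, clamped to MaxHealth.
; Looping timers started at BeginPlay spin the mesh, pull the actor toward a nearby player and steadily shrink it until it destroys itself.
; On overlap with BP_Player it calls SaveBuff, applies the heal, plays a pickup sound and destroys itself.
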(event `self.ReceiveBeginPlay`
  (`parent.ReceiveBeginPlay`)
  (`KismetSystemLibrary.K2_SetTimerDelegate` (delegate `Rotation`) 0.01 true)
  (set `self.Player` (`GameplayStatics.GetPlayerCharacter` 0))
  (`KismetSystemLibrary.K2_SetTimerDelegate` (delegate `PullToPlayer`) 0.02 true)
  (`KismetSystemLibrary.K2_SetTimerDelegate` (delegate `Shrink`) 0.01 true))

(event `Rotation`
  (`SceneComponent.K2_AddLocalRotation` (`self.HealthPickup`) (struct :`Yaw` -2.0) false false))

(event `PullToPlayer`
  (bind _player (`self.Player`))
  (`/Engine/EditorBlueprintResources/StandardMacros.IsValid` _player
    (:`Is Valid`
      (if (<= (`self.GetDistanceTo` _player) 500.0)
        (`self.K2_AddActorWorldOffset` (* (`KismetMathLibrary.Normal` (- (`self.K2_GetActorLocation` _player) (`self.K2_GetActorLocation`))) (`GameplayStatics.GetWorldDeltaSeconds`) (`self.AttractSpeed`)))))))

(event `Shrink`
  (bind _returnvalue (- (`self.Scale`) 0.0001))
  (bind _output_get (set `self.Scale` _returnvalue))
  (`SceneComponent.SetWorldScale3D` (`self.DefaultSceneRoot`) (`KismetMathLibrary.Conv_DoubleToVector` _output_get))
  (if (<= _returnvalue 0.0)
    (`self.K2_DestroyActor`)))

(event `self.HealthPickup.OnComponentBeginOverlap`
  (params (OverlappedComponent :type "PrimitiveComponent Object Reference") (OtherActor :type "Actor Object Reference") (OtherComp :type "PrimitiveComponent Object Reference") (OtherBodyIndex :type Integer) (bFromSweep :type Boolean) (SweepResult :type "HitResult Structure (by ref)"))
  (bind _asbp_player (cast `/Game/Player/Blueprints/BP_Player` OtherActor))
  (`self.Save Buff`)
  (bind _output_get (set `/Game/Player/Blueprints/BP_Player.Health` (+ (`/Game/Player/Blueprints/BP_Player.Health` _asbp_player) (`self.RestoreAmount`)) _asbp_player))
  (bind _maxhealth (`/Game/Player/Blueprints/BP_Player.MaxHealth` _asbp_player))
  (if (> _output_get _maxhealth)
    (set `/Game/Player/Blueprints/BP_Player.Health` _maxhealth _asbp_player))
  (`GameplayStatics.PlaySoundAtLocation` "/Game/Audio/health_pickup.health_pickup" (`SceneComponent.K2_GetComponentLocation` (`self.DefaultSceneRoot`)) (struct) 1.0 1.0 0.0 null null null null)
  (`self.K2_DestroyActor`))

(fn `UserConstructionScript`)