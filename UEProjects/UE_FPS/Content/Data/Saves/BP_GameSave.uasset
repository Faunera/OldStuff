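; BP_GameSave is a save data Blueprint holding player loadout, progression and settings state.
; It stores weapon classes with transforms and ammo counts, plus health, keys, powerups, walk speed, damage reduction and audio volume.
; ClearSave wipes the stored collections and resets audio volume and damage reduction to their defaults.
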(event `ClearSave`
  (`KismetArrayLibrary.Array_Clear` (`self.WeaponClassReference`))
  (`KismetArrayLibrary.Array_Clear` (`self.WeaponTransforms`))
  (`KismetArrayLibrary.Array_Clear` (`self.CurrentAmmos`))
  (`KismetArrayLibrary.Array_Clear` (`self.MaxAmmos`))
  (`KismetArrayLibrary.Array_Clear` (`self.Health`))
  (`KismetArrayLibrary.Array_Clear` (`self.Keys`))
  (`KismetArrayLibrary.Array_Clear` (`self.Powerups`))
  (set `self.AudioVolume` 100.0)
  (`KismetArrayLibrary.Array_Clear` (`self.WalkSpeed`))
  (set `self.DmgReduction` 0.0))